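; BP_Girl is a dialogue NPC that shows the player lines of text from its Text variable.
; A box overlap with BP_Player reveals a text render and creates a Dialogue_UI widget; leaving hides the text and removes the widget.
; EventDialogue passes Text to the widget, shows it and advances its row index, removing it at the last row, with a DoOnce that is reset after each step.
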(event `self.ReceiveTick`
  (params (DeltaSeconds :type "Float (single-precision)")))

(event `self.Box.OnComponentBeginOverlap`
  (params (OverlappedComponent :type "PrimitiveComponent Object Reference") (OtherActor :type "Actor Object Reference") (OtherComp :type "PrimitiveComponent Object Reference") (OtherBodyIndex :type Integer) (bFromSweep :type Boolean) (SweepResult :type "HitResult Structure (by ref)"))
  (cast `/Game/Blueprints/BP_Player` OtherActor)
  (`SceneComponent.SetHiddenInGame` (`self.TextRender`) false false)
  (bind _returnvalue (`|CreateWidget` "/Game/DialogueSystem/Dialogue_UI.Dialogue_UI_C"))
  (bind _output_get (set `self.DialogueUI` _returnvalue))
  (`UserWidget.AddToViewport` _output_get 0))

(event `self.Box.OnComponentEndOverlap`
  (params (OverlappedComponent :type "PrimitiveComponent Object Reference") (OtherActor :type "Actor Object Reference") (OtherComp :type "PrimitiveComponent Object Reference") (OtherBodyIndex :type Integer))
  (bind _dialogueui (`self.DialogueUI`))
  (cast `/Game/Blueprints/BP_Player` OtherActor)
  (`SceneComponent.SetHiddenInGame` (`self.TextRender`) true false)
  (`/Engine/EditorBlueprintResources/StandardMacros.IsValid` _dialogueui
    (:`Is Valid`
      (`Widget.RemoveFromParent` _dialogueui))))

(event `/Game/DialogueSystem/BPI_DialogueInterface.EventDialogue`
  (bind _dialogueui (`self.DialogueUI`))
  (bind _dialogueui_2 (`self.DialogueUI`))
  (bind _returnvalue (+ (`/Game/DialogueSystem/Dialogue_UI.TextRow` (`self.DialogueUI`)) 1))
  (`/Engine/EditorBlueprintResources/StandardMacros.DoOnce` false :!label _label
    (:`Completed`
      (set `/Game/DialogueSystem/Dialogue_UI.Text` (`self.Text`) _dialogueui)
      (`Widget.SetVisibility` (`/Game/DialogueSystem/Dialogue_UI.TxtDialogue` _dialogueui) "Visible")
      (`Widget.SetVisibility` (`/Game/DialogueSystem/Dialogue_UI.DialogueBorder` _dialogueui) "Visible")
      (if (> _returnvalue (- (`KismetArrayLibrary.Array_Length` (`self.Text`)) 1))
        (`Widget.RemoveFromParent` _dialogueui_2)
        (`self.ResetDoOnce`)
        (else
          (set `/Game/DialogueSystem/Dialogue_UI.TextRow` _returnvalue _dialogueui_2)
          (`self.ResetDoOnce`))))))

(event `ResetDoOnce`
  (goto _label :!via `Reset`))

(fn `UserConstructionScript`)