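; Dialogue component for Fabio, the Mission 2 NPC who briefs the player, in Spanish, on rescuing a disoriented fox with a rope from the lake pier.
; After calling the parent Dialogue, it switches on the active branch: the default plays a chain of lines, each gated on the previous one's Pass Through state.
; The briefing ends by switching to BuscarCuerda, which repeats a reminder to find the rope, clears progress and closes the conversation.
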(fn `Dialogue`
  (`parent.Dialogue`)
  (switch `name` (`self.ActiveDialogueBranch`)
    (:`Default`
      (bind _state (`self.AddDialogue` "Fabio" "¡Tú debes ser el rescatista de fauna silvestre! Soy Fabio, uno de los encargados aquí. Me alegra ver que estés dispuesto a ayudar con la situación del animal salvaje que hemos avistado" (`|MakeArray` "Continuar" :!type "Text")))
      (switch `/Game/Blueprints/Enum_DialogueState` _state
        (:`NewEnumerator0`
          (bind _state_2 (`self.AddDialogue` "Fabio" "Te cuento un poco más sobre el asunto. Resulta que hemos visto a un zorro merodeando cerca de una de nuestras casas del árbol. Parece un poco desorientado y asustado, así que es crucial que lo ayudemos lo antes posible" (`|MakeArray` "Continuar" :!type "Text")))
          (switch `/Game/Blueprints/Enum_DialogueState` _state_2
            (:`NewEnumerator0`
              (bind _state_3 (`self.AddDialogue` "Fabio" "En situaciones como esta, siempre es mejor tener cuidado con la distancia y evitar asustar al animal aún más" (`|MakeArray` "Cuéntame más Carlos" :!type "Text")))
              (switch `/Game/Blueprints/Enum_DialogueState` _state_3
                (:`NewEnumerator0`
                  (bind _state_4 (`self.AddDialogue` "Fabio" "Mi sugerencia es usar una cuerda para poder amarrar al zorro de manera segura y así evitar que se escape o se lastime mientras lo llevamos a un lugar más tranquilo" (`|MakeArray` "Continuar" :!type "Text")))
                  (switch `/Game/Blueprints/Enum_DialogueState` _state_4
                    (:`NewEnumerator0`
                      (bind _state_5 (`self.AddDialogue` "Fabio" "Afortunadamente, tenemos una cuerda justo aquí en el campamento. Está ubicada en el muelle, junto al lago. Con esta, podrás asegurar al zorro y luego evaluar su estado con más calma" (`|MakeArray` "Continuar" :!type "Text")))
                      (switch `/Game/Blueprints/Enum_DialogueState` _state_5
                        (:`NewEnumerator0`
                          (bind _state_6 (`self.AddDialogue` "Fabio" "De esta manera, si está herido o necesita atención médica, podrás trasladarlo de manera segura al Centro de Atención y Valoración de Fauna Silvestre" (`|MakeArray` "Continuar" :!type "Text")))
                          (switch `/Game/Blueprints/Enum_DialogueState` _state_6
                            (:`NewEnumerator0`
                              (`self.AddDialogue` "Fabio" "Confió en ti y sé que harás un trabajo genial " (`|MakeArray` "Continuar" :!type "Text"))
                              (`self.SetDialogueBranch` "BuscarCuerda")
                              (`self.CloseConversation`))))))))))))))
    (:`BuscarCuerda`
      (bind _state_7 (`self.AddDialogue` "Fabio" "Busca la cuerda en el muelle del lago"))
      (switch `/Game/Blueprints/Enum_DialogueState` _state_7
        (:`NewEnumerator0`
          (`self.ClearDialogueProgress`)
          (`self.CloseConversation`))))))