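; Dialogue component for the Mission 2 red fox: a Spanish player monologue that teaches species facts, sedation and safe transport to the CAV.
; Overrides Dialogue as chained AddDialogue steps, switched on the active branch.
; The intro explains three sedatives, then sets the OpcionAnestesia branch for a dosage quiz.
; Wrong doses warn and roll progress back one step; the correct one continues through restraint and loading, then clears progress and closes the conversation.
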(fn `Dialogue`
  (`parent.Dialogue`)
  (switch `name` (`self.ActiveDialogueBranch`)
    (:`Default`
      (bind _state (`self.AddDialogue` "Tú" "¡Ahí está! Es un hermoso zorro rojo, un Vulpes vulpes. Parece estar un poco nervioso, pero necesito asegurarme de su seguridad y bienestar" (`|MakeArray` "Continuar" :!type "Text")))
      (switch `/Game/Blueprints/Enum_DialogueState` _state
        (:`NewEnumerator0`
          (bind _state_2 (`self.AddDialogue` "Tú" "Los zorros rojos son conocidos por su pelaje de color naranja-rojizo y sus hábitos nocturnos. Son cazadores ágiles y versátiles, adaptándose a una variedad de entornos, desde bosques hasta zonas urbanas" (`|MakeArray` "Continuar" :!type "Text")))
          (switch `/Game/Blueprints/Enum_DialogueState` _state_2
            (:`NewEnumerator0`
              (bind _state_3 (`self.AddDialogue` "Tú" "Para tranquilizarlo y manejarlo de manera segura, voy a administrarle una combinación de tres agentes sedantes y anestésicos: xilazina, ketamina y medetomidina" (`|MakeArray` "Continuar" :!type "Text")))
              (switch `/Game/Blueprints/Enum_DialogueState` _state_3
                (:`NewEnumerator0`
                  (bind _state_4 (`self.AddDialogue` "Tú" "La xilazina es un medicamento que ayudará a calmar al zorro y reducir su ansiedad durante el procedimiento" (`|MakeArray` "Continuar" :!type "Text")))
                  (switch `/Game/Blueprints/Enum_DialogueState` _state_4
                    (:`NewEnumerator0`
                      (bind _state_5 (`self.AddDialogue` "Tú" "La ketamina actuará como un agente anestésico disociativo. Este compuesto inducirá una pérdida de la consciencia y del control muscular, permitiendo un manejo seguro del animal durante el transporte" (`|MakeArray` "Continuar" :!type "Text")))
                      (switch `/Game/Blueprints/Enum_DialogueState` _state_5
                        (:`NewEnumerator0`
                          (bind _state_6 (`self.AddDialogue` "Tú" "Por último, la medetomidina se utilizará como un agente sedante adicional. Este medicamento proporcionará una sedación adicional al zorro, ayudando a mantenerlo tranquilo durante el traslado" (`|MakeArray` "Continuar" :!type "Text")))
                          (switch `/Game/Blueprints/Enum_DialogueState` _state_6
                            (:`NewEnumerator1`
                              (`self.SetDialogueBranch` "OpcionAnestesia"))))))))))))))
    (:`OpcionAnestesia`
      (bind _state_7 (`self.AddDialogue` "Tú" "Ahora, debo calcular cuidadosamente las dosis correctas de cada medicamento para asegurar una sedación y anestesia efectivas, pero sin poner en peligro la salud del zorro" (`|MakeArray` "Continuar" :!type "Text")))
      (switch `/Game/Blueprints/Enum_DialogueState` _state_7
        (:`NewEnumerator0`
          (bind (_state_8 _optionindex) (`self.AddDialogue` "Tú" "¿Cuál será la cantidad adecuada para este zorro de pelaje rojo? " (`|MakeArray` "0.5 – 2 mg/kg de xilazina, 5 - 20 mg/kg de Ketamina y 0.05 - 0.1 mg/kg Medetomidina" "2 – 4 mg/kg de xilazina, 20 - 40 mg/kg de Ketamina y 0.1 - 0.5 mg/kg Medetomidina" "3 – 6 mg/kg de xilazina, 30 - 50 mg/kg de Ketamina y 1 - 1.5 mg/kg Medetomidina" :!type "Text")))
          (switch `/Game/Blueprints/Enum_DialogueState` _state_8
            (:`NewEnumerator0`
              (switch `int` _optionindex
                (:`0`
                  (bind _state_9 (`self.AddDialogue` "Tú" "Esta cantidad es la adecuada para anestesiar al zorro de manera segura y efectiva. Su combinación proporciona una sedación y anestesia suficientes para el tamaño y la sensibilidad de esta especie, garantizando un procedimiento seguro de traslado" (`|MakeArray` "Continuar" :!type "Text")))
                  (switch `/Game/Blueprints/Enum_DialogueState` _state_9
                    (:`NewEnumerator0`
                      (bind _state_10 (`self.AddDialogue` "Tú" "Ahora que el zorro esta sedado, procederé a amarrarlo con la cuerda. Es importante hacerlo con cuidado para evitar lastimarlo y garantizar su seguridad durante el transporte al CAV" (`|MakeArray` "Continuar" :!type "Text")))
                      (switch `/Game/Blueprints/Enum_DialogueState` _state_10
                        (:`NewEnumerator0`
                          (bind _state_11 (`self.AddDialogue` "Tú" "Al amarrar al zorro, aseguraré la cuerda alrededor de su torso de manera firme pero no ajustada. Esto permitirá que pueda respirar adecuadamente y moverse con cierta libertad, pero también evitará que se escape o se lastime durante el traslado" (`|MakeArray` "Continuar" :!type "Text")))
                          (switch `/Game/Blueprints/Enum_DialogueState` _state_11
                            (:`NewEnumerator0`
                              (`self.AddDialogue` "Tú" "Una vez que esté completamente asegurado, lo cargaré con cuidado en la parte trasera del vehículo" (`|MakeArray` "Continuar" :!type "Text"))
                              (switch `/Game/Blueprints/Enum_DialogueState` "NewEnumerator0"
                                (:`NewEnumerator0`
                                  (bind _state_12 (`self.AddDialogue` "Tú" "Con este método de transporte, se puede garantizar la seguridad y el bienestar del venado durante todo el viaje hacia el CAV" (`|MakeArray` "Continuar" :!type "Text")))
                                  (switch `/Game/Blueprints/Enum_DialogueState` _state_12
                                    (:`NewEnumerator0`
                                      (bind _state_13 (`self.AddDialogue` "Tú" "¡Buena suerte en el viaje amigo!" (`|MakeArray` "Continuar" :!type "Text")))
                                      (switch `/Game/Blueprints/Enum_DialogueState` _state_13
                                        (:`NewEnumerator0`
                                          (`self.ClearDialogueProgress`)
                                          (`self.CloseConversation`))))))))))))))
                (:`1`
                  (bind _state_14 (`self.AddDialogue` "Tú" "Esta cantidad es demasiado y puede llegar a ser fatal para el zorro" (`|MakeArray` "Continuar" :!type "Text")))
                  (switch `/Game/Blueprints/Enum_DialogueState` _state_14
                    (:`NewEnumerator0`
                      (`self.RemoveDialogueProgress` 1))))
                (:`2`
                  (bind _state_15 (`self.AddDialogue` "Tú" "Esta cantidad es demasiado y puede llegar a ser fatal para el zorro" (`|MakeArray` "Continuar" :!type "Text")))
                  (switch `/Game/Blueprints/Enum_DialogueState` _state_15
                    (:`NewEnumerator0`
                      (`self.RemoveDialogueProgress` 1))))))))))))