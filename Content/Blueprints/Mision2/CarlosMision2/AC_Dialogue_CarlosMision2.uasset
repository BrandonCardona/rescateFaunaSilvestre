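; Dialogue component for the NPC Carlos in Mission 2, holding his Spanish conversation with the player, a new member of the rescue team.
; The default branch welcomes the player and introduces an important mission, then switches to the MisionMansion branch and closes.
; That branch randomly shows either a reminder to rescue the animal at the northwest mansion or an ice cream quip, then clears dialogue progress and closes.
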(fn `Dialogue`
  (`parent.Dialogue`)
  (switch `name` (`self.ActiveDialogueBranch`)
    (:`Default`
      (bind _state (`self.AddDialogue` "Carlos" "¡Hola, compañero rescatista! María me ha contado que te has unido a nuestro equipo, ¡bienvenido!"))
      (switch `/Game/Blueprints/Enum_DialogueState` _state
        (:`NewEnumerator0`
          (bind _state_2 (`self.AddDialogue` "Carlos" "Estoy encantado de tenerte con nosotros. Tenemos una misión muy importante por delante y tu ayuda será fundamental." (`|MakeArray` "Cuéntame Carlos" :!type "Text")))
          (switch `/Game/Blueprints/Enum_DialogueState` _state_2
            (:`NewEnumerator0`
              (`self.SetDialogueBranch` "MisionMansion")
              (`self.CloseConversation`))))))
    (:`MisionMansion`
      (bind _state_3 (`self.AddDialogue` "Carlos" (select `int` (`KismetMathLibrary.RandomIntegerInRange` 0 1) :`0` "Ve a la mansión al noroeste de la ciudad y rescata el animal" :`1` "Se me antojo un helado" :!type "Text") (`|MakeArray`)))
      (switch `/Game/Blueprints/Enum_DialogueState` _state_3
        (:`NewEnumerator0`
          (`self.ClearDialogueProgress`)
          (`self.CloseConversation`))))))