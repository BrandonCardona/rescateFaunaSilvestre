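; Dialogue component for the NPC María in Mission 2, congratulating the player for rescuing a white-tailed deer.
; The default branch chains eight Spanish lines on the animal's scientific name, its transfer to a wildlife care center (CAV) and captivity effects, then directs the player to Carlos.
; It then switches to the BuscarCarlos branch, which repeats the Carlos reminder, clears dialogue progress and closes the conversation on later talks.
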(fn `Dialogue`
  (`parent.Dialogue`)
  (switch `name` (`self.ActiveDialogueBranch`)
    (:`Default`
      (bind _state (`self.AddDialogue` "Maria" "¡Fantástico trabajo! Has demostrado ser un rescatista excepcional al salvar al venado de cola blanca. Estoy realmente impresionada por tu valentía y dedicación para con los animales" (`|MakeArray` "Continuar" :!type "Text")))
      (switch `/Game/Blueprints/Enum_DialogueState` _state
        (:`NewEnumerator0`
          (bind _state_2 (`self.AddDialogue` "María" "Recuerda igualmente que es muy importante referirnos al animal por su nombre científico. En nuestro caso es Odocoileus virginianus" (`|MakeArray` "Continuar" :!type "Text")))
          (switch `/Game/Blueprints/Enum_DialogueState` _state_2
            (:`NewEnumerator0`
              (bind _state_3 (`self.AddDialogue` "María" "Ahora que el animal está a salvo, lo llevaremos al Centro de Atención y valoración de fauna silvestre (CAV) para que reciba el tratamiento y cuidado adecuados" (`|MakeArray` "Continuar" :!type "Text")))
              (switch `/Game/Blueprints/Enum_DialogueState` _state_3
                (:`NewEnumerator0`
                  (bind _state_4 (`self.AddDialogue` "María" "Las personas que lo tuvieron en cautiverio pueden haber afectado significativamente el comportamiento natural del animal" (`|MakeArray` "Continuar" :!type "Text")))
                  (switch `/Game/Blueprints/Enum_DialogueState` _state_4
                    (:`NewEnumerator0`
                      (bind _state_5 (`self.AddDialogue` "María" "La interacción constante con humanos y el entorno artificial pueden haber generado dependencia y desadaptación al medio silvestre. Esto plantea la posibilidad de que el venado ya no sea apto para ser liberado en su hábitat natural" (`|MakeArray` "Continuar" :!type "Text")))
                      (switch `/Game/Blueprints/Enum_DialogueState` _state_5
                        (:`NewEnumerator0`
                          (bind _state_6 (`self.AddDialogue` "María" "Esperemos que nuestros veterinarios logren que se recupere completamente y decidan si será liberado de nuevo en su hábitat natural o definitivamente debe permanecer en cautiverio" (`|MakeArray` "Continuar" :!type "Text")))
                          (switch `/Game/Blueprints/Enum_DialogueState` _state_6
                            (:`NewEnumerator0`
                              (bind _state_7 (`self.AddDialogue` "María" "Por ahora, ve y habla con Carlos para recibir tu próxima misión, debe estar en la heladería cerca al parque" (`|MakeArray` "Continuar" :!type "Text")))
                              (switch `/Game/Blueprints/Enum_DialogueState` _state_7
                                (:`NewEnumerator0`
                                  (bind _state_8 (`self.AddDialogue` "María" "¡Buena suerte y sigue siendo ese increíble defensor de la vida silvestre!" (`|MakeArray` "Continuar" :!type "Text")))
                                  (switch `/Game/Blueprints/Enum_DialogueState` _state_8
                                    (:`NewEnumerator0`
                                      (`self.SetDialogueBranch` "BuscarCarlos")
                                      (`self.CloseConversation`))))))))))))))))))
    (:`BuscarCarlos`
      (bind _state_9 (`self.AddDialogue` "María" "Habla con Carlos en la heladería cerca al parque "))
      (switch `/Game/Blueprints/Enum_DialogueState` _state_9
        (:`NewEnumerator0`
          (`self.ClearDialogueProgress`)
          (`self.CloseConversation`))))))