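; Dialogue component for the second car shortcut (Carro2), offering the player a Spanish-language choice to take a shortcut through the city or stay.
; Overrides Dialogue, calling the parent and then building the branching conversation with AddDialogue.
; Taking the shortcut ends the conversation and moves BP_Player to a hardcoded location.
; Staying shows a short decline line, then clears progress and closes the conversation.
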(fn `Dialogue`
  (`parent.Dialogue`)
  (switch `name` (`self.ActiveDialogueBranch`)
    (:`Default`
      (bind (_state _optionindex) (`self.AddDialogue` "Tu" "Parece que se puede usar el auto para recorrer la ciudad" (`|MakeArray` "Tomar atajo" "Permanecer aquí" :!type "Text")))
      (switch `/Game/Blueprints/Enum_DialogueState` _state
        (:`NewEnumerator0`
          (switch `int` _optionindex
            (:`0`
              (`self.ClearDialogueProgress`)
              (`self.CloseConversation`)
              (bind _asbp_player (cast `/Game/Blueprints/BP_Player` (`GameplayStatics.GetPlayerPawn` 0)))
              (`Actor.K2_SetActorLocation` _asbp_player (1095.0 306.0 56.0) false false))
            (:`1`
              (bind _state_2 (`self.AddDialogue` "Tu" "Será en otro momento"))
              (switch `/Game/Blueprints/Enum_DialogueState` _state_2
                (:`NewEnumerator0`
                  (`self.ClearDialogueProgress`)
                  (`self.CloseConversation`))))))))))