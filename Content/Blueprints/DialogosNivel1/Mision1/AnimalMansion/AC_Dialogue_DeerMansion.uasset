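; Dialogue component for the white-tailed deer at the mansion in Mission 1: an educational Spanish monologue where the player sedates and relocates the animal.
; The Dialogue override chains AddDialogue lines across three branches: species introduction, xylazine/Telazol review, then a dose quiz, advanced via SetDialogueBranch.
; Wrong doses explain the error and step back with RemoveDialogueProgress; the correct one continues into cage transport, then clears progress and closes the conversation.
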(fn `Dialogue`
  (`parent.Dialogue`)
  (switch `name` (`self.ActiveDialogueBranch`)
    (:`Default`
      (bind _state (`self.AddDialogue` "Tú" "¡Vaya, qué belleza! Es un venado de cola blanca, también conocido como Odocoileus virginianus" (`|MakeArray` "Continuar" :!type "Text")))
      (switch `/Game/Blueprints/Enum_DialogueState` _state
        (:`NewEnumerator0`
          (bind _state_2 (`self.AddDialogue` "Tú" "Estoy aquí para ayudarte, amigo. Solo quiero asegurarme de que estés bien y encontrar la mejor manera de llevarte a un lugar seguro" (`|MakeArray` "Continuar" :!type "Text")))
          (switch `/Game/Blueprints/Enum_DialogueState` _state_2
            (:`NewEnumerator0`
              (bind _state_3 (`self.AddDialogue` "Tú" "Los venados de cola blanca son herbívoros al igual que sus parientes de cola marrón y negra, pero suelen habitar en diferentes áreas geográficas, como bosques, praderas y matorrales" (`|MakeArray` "Continuar" :!type "Text")))
              (switch `/Game/Blueprints/Enum_DialogueState` _state_3
                (:`NewEnumerator0`
                  (bind _state_4 (`self.AddDialogue` "Tú" "A diferencia de los venados de cola marrón y negra, los venados de cola blanca suelen ser más grandes en tamaño y tienen una cola distintivamente blanca que levantan cuando están alerta" (`|MakeArray` "Continuar" :!type "Text")))
                  (switch `/Game/Blueprints/Enum_DialogueState` _state_4
                    (:`NewEnumerator0`
                      (bind _state_5 (`self.AddDialogue` "Tú" "No te preocupes, amigo. No estoy aquí para hacerte daño. Solo quiero asegurarme de que estés bien y encontrar la mejor manera de ayudarte" (`|MakeArray` "Continuar" :!type "Text")))
                      (switch `/Game/Blueprints/Enum_DialogueState` _state_5
                        (:`NewEnumerator0`
                          (bind _state_6 (`self.AddDialogue` "Tú" "Debo administrarle un sedante suave para poder trasladarlo a un lugar seguro" (`|MakeArray` "Continuar" :!type "Text")))
                          (switch `/Game/Blueprints/Enum_DialogueState` _state_6
                            (:`NewEnumerator1`
                              (`self.SetDialogueBranch` "Anestesia"))))))))))))))
    (:`OpcionAnestesia`
      (bind _state_7 (`self.AddDialogue` "Tú" "Debo tener cuidado con la cantidad de anestesia que debo administrarle, después de todo, la dosis incorrecta podría ser fatal para él, por lo que hay que ser muy precisos. " (`|MakeArray` "Continuar" :!type "Text")))
      (switch `/Game/Blueprints/Enum_DialogueState` _state_7
        (:`NewEnumerator0`
          (bind (_state_8 _optionindex) (`self.AddDialogue` "Tú" "¿Cuál será la cantidad adecuada para este venado de cola blanca?" (`|MakeArray` "0.5 mg/kg de xilazina y 1 mg/kg de Telazol" "8 mg/kg de xilazina y 16 mg/kg de Telazol" "2.2 mg/kg de xilazina y 4.4 mg/kg de Telazol" :!type "Text")))
          (switch `/Game/Blueprints/Enum_DialogueState` _state_8
            (:`NewEnumerator0`
              (switch `int` _optionindex
                (:`0`
                  (bind _state_9 (`self.AddDialogue` "Tú" "Esta cantidad puede no ser suficiente para anestesiar correctamente al venado" (`|MakeArray` "Continuar" :!type "Text")))
                  (switch `/Game/Blueprints/Enum_DialogueState` _state_9
                    (:`NewEnumerator0`
                      (`self.RemoveDialogueProgress` 1))))
                (:`1`
                  (bind _state_10 (`self.AddDialogue` "Tú" "Esta cantidad es demasiado y puede llegar a ser fatal para el venado" (`|MakeArray` "Continuar" :!type "Text")))
                  (switch `/Game/Blueprints/Enum_DialogueState` _state_10
                    (:`NewEnumerator0`
                      (`self.RemoveDialogueProgress` 1))))
                (:`2`
                  (bind _state_11 (`self.AddDialogue` "Tú" "Esta cantidad es la adecuada para anestesiar al venado de cola blanca de manera segura y efectiva. Su combinación proporciona una sedación y anestesia suficientes para el tamaño y la sensibilidad de esta especie, garantizando un procedimiento seguro de traslado" (`|MakeArray` "Continuar" :!type "Text")))
                  (switch `/Game/Blueprints/Enum_DialogueState` _state_11
                    (:`NewEnumerator0`
                      (bind _state_12 (`self.AddDialogue` "Tú" "Respecto al método de transporte para el venado. Considerando su tamaño y la necesidad de mantenerlo seguro y cómodo durante el traslado, optaremos por una jaula móvil especialmente diseñada para animales de su tamaño" (`|MakeArray` "Continuar" :!type "Text")))
                      (switch `/Game/Blueprints/Enum_DialogueState` _state_12
                        (:`NewEnumerator0`
                          (bind _state_13 (`self.AddDialogue` "Tú" "Estas jaulas proporcionan un espacio adecuado para que el venado pueda estar de pie, acostarse y moverse con comodidad durante el viaje. Está construida con materiales resistentes y cuenta con barras que permiten una buena ventilación" (`|MakeArray` "Continuar" :!type "Text")))
                          (switch `/Game/Blueprints/Enum_DialogueState` _state_13
                            (:`NewEnumerator0`
                              (`self.AddDialogue` "Tú" "Además, la jaula estará asegurada en la parte trasera de una camioneta para garantizar su estabilidad durante el viaje" (`|MakeArray` "Continuar" :!type "Text"))
                              (switch `/Game/Blueprints/Enum_DialogueState` "NewEnumerator0"
                                (:`NewEnumerator0`
                                  (bind _state_14 (`self.AddDialogue` "Tú" "Con este método de transporte, podemos garantizar la seguridad y el bienestar del venado durante todo el viaje hacia el CAV" (`|MakeArray` "Continuar" :!type "Text")))
                                  (switch `/Game/Blueprints/Enum_DialogueState` _state_14
                                    (:`NewEnumerator0`
                                      (bind _state_15 (`self.AddDialogue` "Tú" "¡Buena suerte en el viaje amigo!" (`|MakeArray` "Continuar" :!type "Text")))
                                      (switch `/Game/Blueprints/Enum_DialogueState` _state_15
                                        (:`NewEnumerator0`
                                          (`self.ClearDialogueProgress`)
                                          (`self.CloseConversation`))))))))))))))))))))
    (:`Anestesia`
      (bind _state_16 (`self.AddDialogue` "Tú" "Pero, antes de proceder debería hacer un breve repaso de los medicamentos que voy a utilizar para anestesiarlo." (`|MakeArray` "Continuar" :!type "Text")))
      (switch `/Game/Blueprints/Enum_DialogueState` _state_16
        (:`NewEnumerator0`
          (bind _state_17 (`self.AddDialogue` "Tú" "Primero, la xilazina es un agente sedante y analgésico que se utiliza comúnmente en medicina veterinaria para inducir la sedación y el alivio del dolor en animales. " (`|MakeArray` "Continuar" :!type "Text")))
          (switch `/Game/Blueprints/Enum_DialogueState` _state_17
            (:`NewEnumerator0`
              (bind _state_18 (`self.AddDialogue` "Tú" "Es especialmente efectiva en venados como este, ayudando a reducir la ansiedad y facilitar procedimientos médicos sin causar daño." (`|MakeArray` "Continuar" :!type "Text")))
              (switch `/Game/Blueprints/Enum_DialogueState` _state_18
                (:`NewEnumerator0`
                  (bind _state_19 (`self.AddDialogue` "Tú" "Ahora, va el Telazol. Este es una combinación de dos compuestos: la tiletamina y la zolazepam. Estos dos medicamentos, cuando se combinan, proporcionan un efecto anestésico más completo y prolongado. " (`|MakeArray` "Continuar" :!type "Text")))
                  (switch `/Game/Blueprints/Enum_DialogueState` _state_19
                    (:`NewEnumerator0`
                      (bind _state_20 (`self.AddDialogue` "Tú" "La tiletamina actúa como un anestésico disociativo, lo que significa que induce una pérdida de la consciencia y el control muscular, mientras que la zolazepam actúa como un tranquilizante que prolonga la duración de la anestesia y proporciona analgesia adicional." (`|MakeArray` "Continuar" :!type "Text")))
                      (switch `/Game/Blueprints/Enum_DialogueState` _state_20
                        (:`NewEnumerator0`
                          (bind _state_21 (`self.AddDialogue` "Tú" "La razón por la que se utilizan estos dos medicamentos en combinación es para potenciar sus efectos y asegurar una anestesia segura y efectiva durante el procedimiento. " (`|MakeArray` "Continuar" :!type "Text")))
                          (switch `/Game/Blueprints/Enum_DialogueState` _state_21
                            (:`NewEnumerator0`
                              (bind _state_22 (`self.AddDialogue` "Tú" "La xilazina proporciona la sedación inicial y el alivio del dolor, mientras que el Telazol garantiza una anestesia profunda y prolongada para facilitar el manejo y el transporte del animal." (`|MakeArray` "Continuar" :!type "Text")))
                              (switch `/Game/Blueprints/Enum_DialogueState` _state_22
                                (:`NewEnumerator1`
                                  (`self.SetDialogueBranch` "OpcionAnestesia"))))))))))))))))))