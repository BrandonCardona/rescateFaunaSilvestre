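; Dialogue component for Carlos in level 1, mission 1, who briefs the player on infiltrating a mansion to rescue an illegally held wild animal from a garden maze.
; The default branch plays a linear chain of Spanish lines with occasional player replies, then switches to the MisionMansion branch and closes the conversation.
; That branch gives a random reminder or joke line, then clears dialogue progress and closes.
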(fn `Dialogue`
  (`parent.Dialogue`)
  (switch `name` (`self.ActiveDialogueBranch`)
    (:`Default`
      (bind _state (`self.AddDialogue` "Carlos" "¡Hola, compañero rescatista! María me ha contado que te has unido a nuestro equipo, ¡bienvenido!"))
      (switch `/Game/Blueprints/Enum_DialogueState` _state
        (:`NewEnumerator0`
          (bind _state_2 (`self.AddDialogue` "Carlos" "Estoy encantado de tenerte con nosotros. Tenemos una misión muy importante por delante y tu ayuda será fundamental." (`|MakeArray` "Cuéntame Carlos" :!type "Text")))
          (switch `/Game/Blueprints/Enum_DialogueState` _state_2
            (:`NewEnumerator0`
              (bind _state_3 (`self.AddDialogue` "Carlos" "Verás, hemos recibido un informe sobre una mansión en las afueras de la ciudad. Esta pertenece a una familia adinerada que se rumorea que compra animales de manera ilegal."))
              (switch `/Game/Blueprints/Enum_DialogueState` _state_3
                (:`NewEnumerator0`
                  (bind _state_4 (`self.AddDialogue` "Carlos" "Nos ha llegado información de que tienen en su posesión a un animal silvestre y estamos decididos a rescatarlo. Hay indicios de que lo están manteniendo oculto en un jardín en forma de laberinto en los terrenos de la mansión."))
                  (switch `/Game/Blueprints/Enum_DialogueState` _state_4
                    (:`NewEnumerator0`
                      (bind _state_5 (`self.AddDialogue` "Carlos" "Tu tarea será infiltrarte en la mansión, encontrar este laberinto y rescatar al animal. "))
                      (switch `/Game/Blueprints/Enum_DialogueState` _state_5
                        (:`NewEnumerator0`
                          (bind _state_6 (`self.AddDialogue` "Carlos" "Sabemos que puede ser un desafío, pero confiamos en tus habilidades como rescatista." (`|MakeArray` "Dalo por hecho" :!type "Text")))
                          (switch `/Game/Blueprints/Enum_DialogueState` _state_6
                            (:`NewEnumerator0`
                              (bind _state_7 (`self.AddDialogue` "Carlos" "La mansión está al noroeste de la ciudad. Te recomiendo que te prepares bien antes de ir" (`|MakeArray`)))
                              (switch `/Game/Blueprints/Enum_DialogueState` _state_7
                                (:`NewEnumerator0`
                                  (bind _state_8 (`self.AddDialogue` "Carlos" "¡Buena suerte y que la protección de la vida silvestre esté contigo!"))
                                  (switch `/Game/Blueprints/Enum_DialogueState` _state_8
                                    (:`NewEnumerator0`
                                      (`self.SetDialogueBranch` "MisionMansion")
                                      (`self.CloseConversation`))))))))))))))))))
    (:`MisionMansion`
      (bind _state_9 (`self.AddDialogue` "Carlos" (select `int` (`KismetMathLibrary.RandomIntegerInRange` 0 1) :`0` "Ve a la mansión al noroeste de la ciudad y rescata el animal" :`1` "Se me antojo un helado" :!type "Text") (`|MakeArray`)))
      (switch `/Game/Blueprints/Enum_DialogueState` _state_9
        (:`NewEnumerator0`
          (`self.ClearDialogueProgress`)
          (`self.CloseConversation`))))))