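; Dialogue component for María's level 1 intro, welcoming the player as the new wildlife rescuer and sending them to find Carlos at the ice cream stand.
; It overrides Dialogue, switching on the active branch and chaining AddDialogue lines through their Pass Through state.
; Confirming identity plays the briefing and sets the BuscarCarlos branch; denying it clears progress and closes.
; On that branch, María gives one of two random reminder lines before closing.
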(fn `Dialogue`
  (`parent.Dialogue`)
  (switch `name` (`self.ActiveDialogueBranch`)
    (:`Default`
      (bind (_state _optionindex) (`self.AddDialogue` "Maria" "¡Genial!, tú debes de ser el nuevo rescatista de fauna silvestre" (`|MakeArray` "Sí, soy yo" "Creo que te equivocaste de persona" :!type "Text")))
      (switch `/Game/Blueprints/Enum_DialogueState` _state
        (:`NewEnumerator0`
          (switch `int` _optionindex
            (:`0`
              (bind _state_2 (`self.AddDialogue` "María" "¡Bienvenido al equipo! Me llamo María, es un gusto por fin conocerte" (`|MakeArray`)))
              (switch `/Game/Blueprints/Enum_DialogueState` _state_2
                (:`NewEnumerator0`
                  (bind _state_3 (`self.AddDialogue` "María" "En este rol, nuestro principal objetivo es proteger y rescatar a los animales en peligro. Ya sabes, ¡somos los héroes de las criaturas más vulnerables de nuestro entorno!"))
                  (switch `/Game/Blueprints/Enum_DialogueState` _state_3
                    (:`NewEnumerator0`
                      (bind _state_4 (`self.AddDialogue` "María" "Día a día nos enfrentamos a desafíos constantes, desde animales heridos por cazadores hasta aquellos adquiridos de manera ilegal por las personas"))
                      (switch `/Game/Blueprints/Enum_DialogueState` _state_4
                        (:`NewEnumerator0`
                          (bind _state_5 (`self.AddDialogue` "María" "Pero sé que con tu ayuda, podemos marcar la diferencia y ayudar a estos animales de fauna silvestre"))
                          (switch `/Game/Blueprints/Enum_DialogueState` _state_5
                            (:`NewEnumerator0`
                              (bind _state_6 (`self.AddDialogue` "María" "¿Listo para ponerte en acción y convertirte en un auténtico defensor de la vida silvestre?" (`|MakeArray` "Claro María" :!type "Text")))
                              (switch `/Game/Blueprints/Enum_DialogueState` _state_6
                                (:`NewEnumerator0`
                                  (bind _state_7 (`self.AddDialogue` "María" "¡Perfecto! Debes buscar a Carlos, él te dirá cuál es tu primera misión como rescatista de fauna silvestre " (`|MakeArray`)))
                                  (switch `/Game/Blueprints/Enum_DialogueState` _state_7
                                    (:`NewEnumerator0`
                                      (bind _state_8 (`self.AddDialogue` "María" "Él suele encontrarse en el puesto de helados, justo debajo de la comisaría de policía"))
                                      (switch `/Game/Blueprints/Enum_DialogueState` _state_8
                                        (:`NewEnumerator0`
                                          (bind _state_9 (`self.AddDialogue` "María" "¡Suerte con eso!"))
                                          (switch `/Game/Blueprints/Enum_DialogueState` _state_9
                                            (:`NewEnumerator0`
                                              (`self.SetDialogueBranch` "BuscarCarlos")
                                              (`self.CloseConversation`))))))))))))))))))
            (:`1`
              (bind _state_10 (`self.AddDialogue` "María" "Disculpame, creo que me confundí" (`|MakeArray`)))
              (switch `/Game/Blueprints/Enum_DialogueState` _state_10
                (:`NewEnumerator0`
                  (`self.ClearDialogueProgress`)
                  (`self.CloseConversation`))))))))
    (:`BuscarCarlos`
      (bind _state_11 (`self.AddDialogue` "María" (select `int` (`KismetMathLibrary.RandomIntegerInRange` 0 1) :`0` "Explora la ciudad y habla con Carlos en el puesto de helados" :`1` "¿Por qué le gustará tanto el helado a Carlos?" :!type "Text") (`|MakeArray`)))
      (switch `/Game/Blueprints/Enum_DialogueState` _state_11
        (:`NewEnumerator0`
          (`self.ClearDialogueProgress`)
          (`self.CloseConversation`))))))