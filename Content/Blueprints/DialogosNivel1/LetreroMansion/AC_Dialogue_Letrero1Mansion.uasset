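; Dialogue component for the first mansion sign in Level 1, in which the player reads an anonymous letter about a hidden animal, its keys and wildlife rescuers.
; It overrides Dialogue, calls the parent, then runs a linear chain of AddDialogue lines alternating from the player ("Tu") to "Anónimo" and back.
; Each line advances on Pass Through; the last clears dialogue progress and closes the conversation.
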(fn `Dialogue`
  (`parent.Dialogue`)
  (switch `name` (`self.ActiveDialogueBranch`)
    (:`Default`
      (bind _state (`self.AddDialogue` "Tu" "Parece  que alguien dejo una carta"))
      (switch `/Game/Blueprints/Enum_DialogueState` _state
        (:`NewEnumerator0`
          (bind _state_2 (`self.AddDialogue` "Anónimo " "He dejado el animal al lado del cobertizo al final del jardín"))
          (switch `/Game/Blueprints/Enum_DialogueState` _state_2
            (:`NewEnumerator0`
              (bind _state_3 (`self.AddDialogue` "Anónimo" "Las llaves estan en el mismo lugar de siempre. Con la primera abres la fuente y con la segunda la puerta hacia el animal. "))
              (switch `/Game/Blueprints/Enum_DialogueState` _state_3
                (:`NewEnumerator0`
                  (bind _state_4 (`self.AddDialogue` "Anónimo" "Hay que tener cuidado y ser discretos. Escuche que esos rescatistas de fauna ya saben del animal y quieren llevarselo"))
                  (switch `/Game/Blueprints/Enum_DialogueState` _state_4
                    (:`NewEnumerator0`
                      (bind _state_5 (`self.AddDialogue` "Anónimo" "No pienso dejar que eso suceda"))
                      (switch `/Game/Blueprints/Enum_DialogueState` _state_5
                        (:`NewEnumerator0`
                          (bind _state_6 (`self.AddDialogue` "Tu" "Qué caso"))
                          (switch `/Game/Blueprints/Enum_DialogueState` _state_6
                            (:`NewEnumerator0`
                              (`self.ClearDialogueProgress`)
                              (`self.CloseConversation`))))))))))))))))