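; Paper2D bear that walks continuously along its forward vector, turning back whenever its walk detector overlaps something.
; Tick feeds forward movement input and picks the up or reversed-down flipbook from the sign of Y velocity.
; A WalkDetector begin-overlap calls TurnChar, which rotates the actor 180 degrees without filtering what it touched.
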(event `self.ReceiveTick`
  (params (DeltaSeconds :type "Float (single-precision)"))
  (bind (_returnvalue_x _returnvalue_y) (`KismetMathLibrary.BreakVector` (`self.GetVelocity`)))
  (`self.AddMovementInput` (`self.GetActorForwardVector`))
  (if (>= _returnvalue_y 0.0)
    (`PaperFlipbookComponent.SetFlipbook` (`self.Sprite`) "/Game/Assets/Animals/Bear/Down/Bear_DownReverse.Bear_DownReverse")
    (else
      (`PaperFlipbookComponent.SetFlipbook` (`self.Sprite`) "/Game/Assets/Animals/Bear/Up/Bear_Up.Bear_Up"))))

(event `self.WalkDetector.OnComponentBeginOverlap`
  (params (OverlappedComponent :type "PrimitiveComponent Object Reference") (OtherActor :type "Actor Object Reference") (OtherComp :type "PrimitiveComponent Object Reference") (OtherBodyIndex :type Integer) (bFromSweep :type Boolean) (SweepResult :type "HitResult Structure (by ref)"))
  (`self.TurnChar`))

(fn `TurnChar`
  (locals (Giro :type "Rotator Structure" :default (struct)))
  (`self.K2_SetActorRotation` (`KismetMathLibrary.ComposeRotators` (`self.K2_GetActorRotation`) (struct :`Yaw` 180.0))))

(fn `UserConstructionScript`)