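; Dialogue component for María at the end of Mission 3, congratulating the player on rescuing a hyacinth macaw and sending them to a wildlife care center (CAV).
; The default branch chains seven Spanish lines, each with a Continue option, announcing a bus near the police station, then sets the "viajarCAV" branch and closes the conversation.
; That branch repeats a short reminder to take the bus, clears dialogue progress and closes.
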(fn `Dialogue`
  (`parent.Dialogue`)
  (switch `name` (`self.ActiveDialogueBranch`)
    (:`Default`
      (bind _state (`self.AddDialogue` "Maria" "¡Increíble trabajo, rescatista! Estoy realmente impresionada por tu dedicación y profesionalismo al manejar la situación con el animal. Has demostrado una vez más ser un verdadero héroe para estas criaturas vulnerables" (`|MakeArray` "Continuar" :!type "Text")))
      (switch `/Game/Blueprints/Enum_DialogueState` _state
        (:`NewEnumerator0`
          (bind _state_2 (`self.AddDialogue` "María" "Los Anodorhynchus hyacinthinus, también conocidos como guacamayos jacintos, son realmente majestuosos con su plumaje azul intenso y su presencia imponente. Tu manejo cuidadoso y compasivo del ave en esta situación delicada es digno de admiración" (`|MakeArray` "Continuar" :!type "Text")))
          (switch `/Game/Blueprints/Enum_DialogueState` _state_2
            (:`NewEnumerator0`
              (bind _state_3 (`self.AddDialogue` "María" "Después de esta hazaña, creo que es hora de que veas por tus propios ojos cómo es el proceso en un Centro de Atención y Valoración de Fauna Silvestre (CAV)" (`|MakeArray` "Continuar" :!type "Text")))
              (switch `/Game/Blueprints/Enum_DialogueState` _state_3
                (:`NewEnumerator0`
                  (bind _state_4 (`self.AddDialogue` "María" "Es crucial para un rescatista comprender completamente el ciclo de cuidado y rehabilitación de estos animales para poder seguir haciendo una diferencia significativa en su vida" (`|MakeArray` "Continuar" :!type "Text")))
                  (switch `/Game/Blueprints/Enum_DialogueState` _state_4
                    (:`NewEnumerator0`
                      (bind _state_5 (`self.AddDialogue` "María" "Por eso, he organizado un autobús que te estará esperando cerca a la estación de policía. Nos dirigiremos hacia un CAV al este de la ciudad, donde podrás presenciar de primera mano cómo se cuida, trata y rehabilita a la fauna silvestre que necesita nuestra ayuda" (`|MakeArray` "Continuar" :!type "Text")))
                      (switch `/Game/Blueprints/Enum_DialogueState` _state_5
                        (:`NewEnumerator0`
                          (bind _state_6 (`self.AddDialogue` "María" "Este será un viaje educativo y emocionante, donde podrás aprender más sobre el importante trabajo que se realiza en estos centros y cómo tu labor como rescatista contribuye a la protección y conservación de la vida silvestre" (`|MakeArray` "Continuar" :!type "Text")))
                          (switch `/Game/Blueprints/Enum_DialogueState` _state_6
                            (:`NewEnumerator0`
                              (bind _state_7 (`self.AddDialogue` "María" "¡Así que prepárate para esta experiencia única, rescatista! El autobús está listo para partir, y estoy segura de que será una experiencia enriquecedora para ti. ¡Vamos a seguir siendo esos increíbles defensores de la vida silvestre juntos!" (`|MakeArray` "Continuar" :!type "Text")))
                              (switch `/Game/Blueprints/Enum_DialogueState` _state_7
                                (:`NewEnumerator0`
                                  (`self.SetDialogueBranch` "viajarCAV")
                                  (`self.CloseConversation`))))))))))))))))
    (:`viajarCAV`
      (bind _state_8 (`self.AddDialogue` "María" "Ve al autobús cerca a la estación de policía y viaja al CAV"))
      (switch `/Game/Blueprints/Enum_DialogueState` _state_8
        (:`NewEnumerator0`
          (`self.ClearDialogueProgress`)
          (`self.CloseConversation`))))))