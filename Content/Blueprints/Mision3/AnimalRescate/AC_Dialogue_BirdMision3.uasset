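; Dialogue component for the Mission 3 animal rescue, a Spanish player monologue on sedating and transporting a blue macaw.
; The Dialogue override chains AddDialogue calls by their returned state, moving from an educational intro to the OpcionAnestesia branch.
; There a three-option dosage quiz rewinds one progress step on either wrong answer.
; The correct middle option leads through cage and transport lines, then clears progress and closes the conversation.
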(fn `Dialogue`
  (`parent.Dialogue`)
  (switch `name` (`self.ActiveDialogueBranch`)
    (:`Default`
      (bind _state (`self.AddDialogue` "Tú" "¡Vaya, eres una guacamaya azul! Anodorhynchus hyacinthinus, Eres realmente imponente con ese plumaje azul intenso y esa cola larga y elegante" (`|MakeArray` "Continuar" :!type "Text")))
      (switch `/Game/Blueprints/Enum_DialogueState` _state
        (:`NewEnumerator0`
          (bind _state_2 (`self.AddDialogue` "Tú" "Pareces estar un poco nerviosa, ¿verdad? No te preocupes, estoy aquí para ayudarte. Mi objetivo es asegurarme de que estés bien y encontrar la mejor manera de llevarte a un lugar seguro" (`|MakeArray` "Continuar" :!type "Text")))
          (switch `/Game/Blueprints/Enum_DialogueState` _state_2
            (:`NewEnumerator0`
              (bind _state_3 (`self.AddDialogue` "Tú" "Las guacamayas azules, también conocidas como guacamayas jacintos, son las aves más grandes del género Anodorhynchus y se distinguen por su color azul vibrante y su pico robusto. Son nativas de América del Sur, principalmente de las selvas tropicales de Brasil, actualmente en peligro de extinción" (`|MakeArray` "Continuar" :!type "Text")))
              (switch `/Game/Blueprints/Enum_DialogueState` _state_3
                (:`NewEnumerator0`
                  (bind _state_4 (`self.AddDialogue` "Tú" "Para asegurar tu comodidad y seguridad durante el traslado, voy a administrarte una combinación de sedantes y anestésicos. En este caso, utilizaré una mezcla de xilazina y ketamina" (`|MakeArray` "Continuar" :!type "Text")))
                  (switch `/Game/Blueprints/Enum_DialogueState` _state_4
                    (:`NewEnumerator0`
                      (bind _state_5 (`self.AddDialogue` "Tú" "La xilazina es un agente sedante que ayudará a reducir tu ansiedad y facilitará el manejo durante el traslado" (`|MakeArray` "Continuar" :!type "Text")))
                      (switch `/Game/Blueprints/Enum_DialogueState` _state_5
                        (:`NewEnumerator0`
                          (bind _state_6 (`self.AddDialogue` "Tú" "Por otro lado, la ketamina actúa como un anestésico disociativo, induciendo una pérdida de la consciencia y del control muscular, lo que te mantendrá tranquila y permitirá un manejo seguro" (`|MakeArray` "Continuar" :!type "Text")))
                          (switch `/Game/Blueprints/Enum_DialogueState` _state_6
                            (:`NewEnumerator1`
                              (`self.SetDialogueBranch` "OpcionAnestesia"))))))))))))))
    (:`OpcionAnestesia`
      (bind _state_7 (`self.AddDialogue` "Tú" "Ahora, debo calcular cuidadosamente las dosis correctas de cada medicamento para asegurar una sedación y anestesia efectivas, pero sin poner en peligro la salud del ave" (`|MakeArray` "Continuar" :!type "Text")))
      (switch `/Game/Blueprints/Enum_DialogueState` _state_7
        (:`NewEnumerator0`
          (bind (_state_8 _optionindex) (`self.AddDialogue` "Tú" "¿Cuál será la cantidad adecuada para este guacamayo azul? " (`|MakeArray` "0.5 – 2 mg/kg de xilazina, 5 - 20 mg/kg de Ketamina y 0.05 - 0.1 mg/kg Medetomidina" "2 – 4 mg/kg de xilazina y 1 - 2 mg/kg de Ketamina " "3 – 6 mg/kg de xilazina, 30 - 50 mg/kg de Ketamina y 1 - 1.5 mg/kg Medetomidina" :!type "Text")))
          (switch `/Game/Blueprints/Enum_DialogueState` _state_8
            (:`NewEnumerator0`
              (switch `int` _optionindex
                (:`0`
                  (bind _state_9 (`self.AddDialogue` "Tú" "Esta cantidad puede no ser suficiente para anestesiar correctamente el ave " (`|MakeArray` "Continuar" :!type "Text")))
                  (switch `/Game/Blueprints/Enum_DialogueState` _state_9
                    (:`NewEnumerator0`
                      (`self.RemoveDialogueProgress` 1))))
                (:`1`
                  (bind _state_10 (`self.AddDialogue` "Tú" "Esta cantidad es la adecuada para anestesiar al zorro de manera segura y efectiva. Su combinación proporciona una sedación y anestesia suficientes para el tamaño y la sensibilidad de esta especie, garantizando un procedimiento seguro de traslado" (`|MakeArray` "Continuar" :!type "Text")))
                  (switch `/Game/Blueprints/Enum_DialogueState` _state_10
                    (:`NewEnumerator0`
                      (bind _state_11 (`self.AddDialogue` "Tú" "Ahora, debo llevar con cuidado el animal a la jaula que nos han prestado. Es espaciosa y segura, diseñada para garantizar su comodidad durante el transporte" (`|MakeArray` "Continuar" :!type "Text")))
                      (switch `/Game/Blueprints/Enum_DialogueState` _state_11
                        (:`NewEnumerator0`
                          (bind _state_12 (`self.AddDialogue` "Tú" "Después se debe preparar el transporte. La jaula estará bien sujeta en el vehículo para evitar movimientos bruscos que puedan asustar al animal" (`|MakeArray` "Continuar" :!type "Text")))
                          (switch `/Game/Blueprints/Enum_DialogueState` _state_12
                            (:`NewEnumerator0`
                              (`self.AddDialogue` "Tú" "Con este método de transporte, se puede garantizar la seguridad y el bienestar del venado durante todo el viaje hacia el CAV" (`|MakeArray` "Continuar" :!type "Text"))
                              (switch `/Game/Blueprints/Enum_DialogueState` "NewEnumerator0"
                                (:`NewEnumerator0`
                                  (bind _state_13 (`self.AddDialogue` "Tú" "¡Buena suerte en el viaje amigo!" (`|MakeArray` "Continuar" :!type "Text")))
                                  (switch `/Game/Blueprints/Enum_DialogueState` _state_13
                                    (:`NewEnumerator0`
                                      (`self.ClearDialogueProgress`)
                                      (`self.CloseConversation`))))))))))))
                (:`2`
                  (bind _state_14 (`self.AddDialogue` "Tú" "Esta cantidad es demasiado y puede llegar a ser fatal para el ave" (`|MakeArray` "Continuar" :!type "Text")))
                  (switch `/Game/Blueprints/Enum_DialogueState` _state_14
                    (:`NewEnumerator0`
                      (`self.RemoveDialogueProgress` 1))))))))))))