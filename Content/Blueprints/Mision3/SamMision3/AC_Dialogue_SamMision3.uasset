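; Dialogue component for Sam in Mission 3, who briefs the player in Spanish on rescuing a hostile blue macaw at a school.
; The default branch chains six lines explaining that Sarah, at the pool, holds the soccer field keys, then switches to the BuscarSarah branch.
; That branch gives a short reminder to talk to Sarah, clears dialogue progress and closes the conversation.
; Sam's handover of pool keys is only spoken; no item is granted here.
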(fn `Dialogue`
  (`parent.Dialogue`)
  (switch `name` (`self.ActiveDialogueBranch`)
    (:`Default`
      (bind _state (`self.AddDialogue` "Sam" "¡Bienvenido, rescatista de fauna silvestre! Es un placer recibirte en nuestra institución. Agradezco enormemente tu disposición para ayudarnos con esta situación tan delicada" (`|MakeArray` "Continuar" :!type "Text")))
      (switch `/Game/Blueprints/Enum_DialogueState` _state
        (:`NewEnumerator0`
          (bind _state_2 (`self.AddDialogue` "Sam" "Permíteme explicarte un poco más sobre la situación con la guacamaya azul. Esta hermosa ave solía ser bastante amigable con los humanos, incluso era la mascota favorita de nuestros estudiantes. Sin embargo, en los últimos días, su comportamiento ha cambiado drásticamente y se ha vuelto hostil sin motivo aparente" (`|MakeArray` "Continuar" :!type "Text")))
          (switch `/Game/Blueprints/Enum_DialogueState` _state_2
            (:`NewEnumerator0`
              (bind _state_3 (`self.AddDialogue` "Sam" "Nos preocupa la seguridad de nuestros alumnos y del propio animal, por lo que es imperativo que intervengamos de manera rápida y efectiva para resolver esta situación" (`|MakeArray` "Continuar" :!type "Text")))
              (switch `/Game/Blueprints/Enum_DialogueState` _state_3
                (:`NewEnumerator0`
                  (bind _state_4 (`self.AddDialogue` "Sam" "Para acceder al área donde se encuentra el ave, necesitarás las llaves del campo de fútbol, ya que la guacamaya se ha refugiado allí. Sarah es la encargada de deportes, quien tiene acceso a las llaves y se encuentra en la piscina del colegio" (`|MakeArray` "Continuar" :!type "Text")))
                  (switch `/Game/Blueprints/Enum_DialogueState` _state_4
                    (:`NewEnumerator0`
                      (bind _state_5 (`self.AddDialogue` "Sam" "Te entregaré las llaves para que puedas acceder a la piscina, ya que Sarah suele dejar la entrada con seguro. Por favor, toma todas las precauciones necesarias para garantizar tu seguridad y la del animal" (`|MakeArray` "Continuar" :!type "Text")))
                      (switch `/Game/Blueprints/Enum_DialogueState` _state_5
                        (:`NewEnumerator0`
                          (bind _state_6 (`self.AddDialogue` "Sam" "Espero que puedas resolver esta situación de manera exitosa y segura. ¡Buena suerte en tu misión, rescatista!" (`|MakeArray` "Continuar" :!type "Text")))
                          (switch `/Game/Blueprints/Enum_DialogueState` _state_6
                            (:`NewEnumerator0`
                              (`self.SetDialogueBranch` "BuscarSarah")
                              (`self.CloseConversation`))))))))))))))
    (:`BuscarSarah`
      (bind _state_7 (`self.AddDialogue` "Sam" "Habla con Sarah en la piscina"))
      (switch `/Game/Blueprints/Enum_DialogueState` _state_7
        (:`NewEnumerator0`
          (`self.ClearDialogueProgress`)
          (`self.CloseConversation`))))))