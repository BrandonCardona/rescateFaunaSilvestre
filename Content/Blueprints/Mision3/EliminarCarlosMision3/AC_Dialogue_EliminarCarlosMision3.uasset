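; Dialogue component for Mission 3 (EliminarCarlos) that asks the player where to go, offering "Colegio" (school) or "Calle" (street).
; It overrides Dialogue, calling the parent first, then adds the line and branches on the selected option index.
; Either choice clears dialogue progress, closes the conversation and moves BP_Player to that option's hard-coded world location without sweeping.
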(fn `Dialogue`
  (`parent.Dialogue`)
  (switch `name` (`self.ActiveDialogueBranch`)
    (:`Default`
      (bind (_state _optionindex) (`self.AddDialogue` "Tú" "¿A donde voy?" (`|MakeArray` "Colegio" "Calle" :!type "Text")))
      (switch `/Game/Blueprints/Enum_DialogueState` _state
        (:`NewEnumerator0`
          (switch `int` _optionindex
            (:`0`
              (`self.ClearDialogueProgress`)
              (`self.CloseConversation`)
              (bind _asbp_player (cast `/Game/Blueprints/BP_Player` (`GameplayStatics.GetPlayerPawn` 0)))
              (`Actor.K2_SetActorLocation` _asbp_player (3737.0 306.0 56.0) false false))
            (:`1`
              (`self.ClearDialogueProgress`)
              (`self.CloseConversation`)
              (bind _asbp_player_2 (cast `/Game/Blueprints/BP_Player` (`GameplayStatics.GetPlayerPawn` 0)))
              (`Actor.K2_SetActorLocation` _asbp_player_2 (3691.0 306.0 56.0) false false))))))))