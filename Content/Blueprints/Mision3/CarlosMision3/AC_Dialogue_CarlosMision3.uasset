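; Dialogue component for Carlos in mission 3, who briefs the rescuer on an aggressive blue macaw at a school northeast of the city.
; A linear AddDialogue chain, run per active dialogue branch, ends in a choice to accept or go prepare.
; Accepting spawns BP_TPColegioIda at a fixed location and switches to the MisionColegio branch, which repeats a short reminder.
; Declining rewinds dialogue progress and closes the conversation.
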(fn `Dialogue`
  (`parent.Dialogue`)
  (switch `name` (`self.ActiveDialogueBranch`)
    (:`Default`
      (bind _state (`self.AddDialogue` "Carlos" "¡Hola de nuevo, compañero rescatista! ¡Qué emocionante es verte de nuevo después de tus heroicas hazañas!" (`|MakeArray` "Continuar" :!type "Text")))
      (switch `/Game/Blueprints/Enum_DialogueState` _state
        (:`NewEnumerator0`
          (bind _state_2 (`self.AddDialogue` "Carlos" "Tenemos una nueva misión que requiere tu valentía y habilidades excepcionales. Esta vez, nos dirigimos a un colegio en las afueras de la ciudad" (`|MakeArray` "Continuar" :!type "Text")))
          (switch `/Game/Blueprints/Enum_DialogueState` _state_2
            (:`NewEnumerator0`
              (bind _state_3 (`self.AddDialogue` "Carlos" "Hemos recibido un informe preocupante sobre una guacamaya azul que actúa de manera agresiva y ha intentado lastimar a los alumnos" (`|MakeArray` "Cuéntame más Carlos" :!type "Text")))
              (switch `/Game/Blueprints/Enum_DialogueState` _state_3
                (:`NewEnumerator0`
                  (bind _state_4 (`self.AddDialogue` "Carlos" "Parece que esta hermosa ave está pasando por un momento difícil, y es crucial que intervengamos para garantizar la seguridad tanto de los estudiantes como del propio animal" (`|MakeArray` "Continuar" :!type "Text")))
                  (switch `/Game/Blueprints/Enum_DialogueState` _state_4
                    (:`NewEnumerator0`
                      (bind _state_5 (`self.AddDialogue` "Carlos" "Tu primera tarea será hablar con el rector del colegio. Él tendrá más información sobre el comportamiento de la guacamaya y las circunstancias que rodean su situación. Es importante entender la situación completamente para poder planificar un rescate seguro y efectivo" (`|MakeArray` "Continuar" :!type "Text")))
                      (switch `/Game/Blueprints/Enum_DialogueState` _state_5
                        (:`NewEnumerator0`
                          (bind (_state_6 _optionindex) (`self.AddDialogue` "Carlos" "El colegio se encuentra al noreste de la ciudad. Te recomiendo que te prepares bien antes de ir, ya que enfrentarás un desafío único y delicado" (`|MakeArray` "Estoy listo" "Necesito prepararme" :!type "Text")))
                          (switch `/Game/Blueprints/Enum_DialogueState` _state_6
                            (:`NewEnumerator0`
                              (switch `int` _optionindex
                                (:`0`
                                  (bind _state_7 (`self.AddDialogue` "Carlos" "¡Confiamos en ti para manejar esta situación con tu profesionalismo y dedicación habituales! ¡Buena suerte en esta nueva misión, rescatista!"))
                                  (switch `/Game/Blueprints/Enum_DialogueState` _state_7
                                    (:`NewEnumerator0`
                                      (`|SpawnActorFromClass` "/Game/Blueprints/Teleports/TPNivel1/BP_TPColegioIda.BP_TPColegioIda_C" (`KismetMathLibrary.MakeTransform` (3128.0 265.0 20.0)) "Undefined" "MultiplyWithRoot" null null)
                                      (`self.SetDialogueBranch` "MisionColegio")
                                      (`self.CloseConversation`))))
                                (:`1`
                                  (bind _state_8 (`self.AddDialogue` "Carlos" "Entiendo, te estare esperando"))
                                  (switch `/Game/Blueprints/Enum_DialogueState` _state_8
                                    (:`NewEnumerator0`
                                      (`self.RemoveDialogueProgress` 2)
                                      (`self.CloseConversation`))))))))))))))))))
    (:`MisionColegio`
      (bind _state_9 (`self.AddDialogue` "Carlos" "Ve al colegio al noreste de la ciudad y rescata el animal"))
      (switch `/Game/Blueprints/Enum_DialogueState` _state_9
        (:`NewEnumerator0`
          (`self.ClearDialogueProgress`)
          (`self.CloseConversation`))))))