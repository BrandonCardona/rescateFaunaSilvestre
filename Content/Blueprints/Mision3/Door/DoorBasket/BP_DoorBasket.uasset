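; BP_DoorBasket is a locked door in Mision3 that moves the player between two fixed positions instead of opening.
; PickUpKey sets HasKey, which gates Interact.
; Each successful Interact alternates through a FlipFlop, teleporting the player pawn to one of two hardcoded world locations regardless of which side they stand on.
; The MostrarNombre overlap volume shows and hides a TextRender label.
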(event `self.Interact`
  (bind _returnvalue (`GameplayStatics.GetPlayerPawn` 0))
  (bind _returnvalue_2 (`GameplayStatics.GetPlayerPawn` 0))
  (if (`self.HasKey?`)
    (`/Engine/EditorBlueprintResources/StandardMacros.FlipFlop`
      (:`A`
        (cast `/Game/Blueprints/BP_Player` _returnvalue_2)
        (`self.K2_SetActorLocation` _returnvalue_2 (4655.0 -264.0 50.0) false false))
      (:`B`
        (cast `/Game/Blueprints/BP_Player` _returnvalue)
        (`self.K2_SetActorLocation` _returnvalue (4655.0 -174.0 50.0) false false)))))

(event `self.PickUpKey`
  (set `self.HasKey?` true))

(event `self.mostrarNombre.OnComponentBeginOverlap`
  (params (OverlappedComponent :type "PrimitiveComponent Object Reference") (OtherActor :type "Actor Object Reference") (OtherComp :type "PrimitiveComponent Object Reference") (OtherBodyIndex :type Integer) (bFromSweep :type Boolean) (SweepResult :type "HitResult Structure (by ref)"))
  (`SceneComponent.SetVisibility` (`self.TextRender`) true false))

(event `self.mostrarNombre.OnComponentEndOverlap`
  (params (OverlappedComponent :type "PrimitiveComponent Object Reference") (OtherActor :type "Actor Object Reference") (OtherComp :type "PrimitiveComponent Object Reference") (OtherBodyIndex :type Integer))
  (`SceneComponent.SetVisibility` (`self.TextRender`) false false))

(fn `UserConstructionScript`)