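; Dialogue component for María in Mission 3 of a wildlife-rescue game, overriding the parent Dialogue graph and switching on the active branch.
; The default branch plays five chained Spanish lines praising the red fox rescue, sharing fox facts and sending the player to Carlos at the supermarket.
; It then sets the BuscarCarlos branch and closes the conversation.
; That branch repeats a short reminder, clearing dialogue progress before closing.
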(fn `Dialogue`
  (`parent.Dialogue`)
  (switch `name` (`self.ActiveDialogueBranch`)
    (:`Default`
      (bind _state (`self.AddDialogue` "Maria" "¡Increíble trabajo, rescatista! Has demostrado una vez más tu valentía y habilidades excepcionales al rescatar el zorro rojo. Realmente has sido un héroe para esta criatura salvaje" (`|MakeArray` "Continuar" :!type "Text")))
      (switch `/Game/Blueprints/Enum_DialogueState` _state
        (:`NewEnumerator0`
          (bind _state_2 (`self.AddDialogue` "María" "Los zorros rojos, también conocidos como Vulpes vulpes, son fascinantes por su adaptabilidad y astucia. Son conocidos por su capacidad para sobrevivir en una amplia variedad de entornos, desde bosques hasta áreas urbanas, y su pelaje naranja-rojizo los hace realmente llamativos" (`|MakeArray` "Continuar" :!type "Text")))
          (switch `/Game/Blueprints/Enum_DialogueState` _state_2
            (:`NewEnumerator0`
              (bind _state_3 (`self.AddDialogue` "María" "Estoy impresionada por cómo manejaste la situación con tanto cuidado y profesionalismo, garantizando la seguridad y el bienestar del zorro en todo momento" (`|MakeArray` "Continuar" :!type "Text")))
              (switch `/Game/Blueprints/Enum_DialogueState` _state_3
                (:`NewEnumerator0`
                  (bind _state_4 (`self.AddDialogue` "María" "Por ahora, tu próxima misión te espera. Debes dirigirte al supermercado cerca de donde nos conocimos. Allí encontrarás a Carlos, quien te informará sobre tu próxima tarea como rescatista de fauna silvestre" (`|MakeArray` "Continuar" :!type "Text")))
                  (switch `/Game/Blueprints/Enum_DialogueState` _state_4
                    (:`NewEnumerator0`
                      (bind _state_5 (`self.AddDialogue` "María" "Sigue siendo ese increíble defensor de la vida silvestre que has demostrado ser, ¡y buena suerte en tu próxima aventura!" (`|MakeArray` "Continuar" :!type "Text")))
                      (switch `/Game/Blueprints/Enum_DialogueState` _state_5
                        (:`NewEnumerator0`
                          (`self.SetDialogueBranch` "BuscarCarlos")
                          (`self.CloseConversation`))))))))))))
    (:`BuscarCarlos`
      (bind _state_6 (`self.AddDialogue` "María" "Habla con Carlos afuera del supermercado"))
      (switch `/Game/Blueprints/Enum_DialogueState` _state_6
        (:`NewEnumerator0`
          (`self.ClearDialogueProgress`)
          (`self.CloseConversation`))))))