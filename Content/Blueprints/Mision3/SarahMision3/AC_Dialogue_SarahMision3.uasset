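; Dialogue component for Sarah in Mission 3, who offers the player a cage for transporting a blue macaw and points to the basketball court, in Spanish.
; Overrides Dialogue, switching on the active branch: the default plays four chained lines, then sets the BuscarJaula branch and closes.
; That branch repeats a short reminder, clears progress and closes.
; Soccer-court keys are only mentioned in text; later intro lines label the speaker "Sam".
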(fn `Dialogue`
  (`parent.Dialogue`)
  (switch `name` (`self.ActiveDialogueBranch`)
    (:`Default`
      (bind _state (`self.AddDialogue` "Sarah" "¡Hola! Veo que estás aquí por la situación con la guacamaya azul. Escuché sobre lo que está sucediendo y quiero ayudar en lo que pueda" (`|MakeArray` "Continuar" :!type "Text")))
      (switch `/Game/Blueprints/Enum_DialogueState` _state
        (:`NewEnumerator0`
          (bind _state_2 (`self.AddDialogue` "Sam" "Sí requieres una jaula para transportar el animal tenemos una disponible justo en la cancha de básquetbol. La preparamos por si necesitábamos trasladar al ave de manera segura. Si la necesitas, estoy más que dispuesta a prestártela" (`|MakeArray` "¡Eso sería genial! " :!type "Text")))
          (switch `/Game/Blueprints/Enum_DialogueState` _state_2
            (:`NewEnumerator0`
              (bind _state_3 (`self.AddDialogue` "Sam" "Por supuesto. La cancha está a unos minutos caminando desde aquí. Verás la jaula cerca de la entrada. También, aquí tienes las llaves para la cancha de Futbol" (`|MakeArray` "Continuar" :!type "Text")))
              (switch `/Game/Blueprints/Enum_DialogueState` _state_3
                (:`NewEnumerator0`
                  (bind _state_4 (`self.AddDialogue` "Sam" "Estoy aquí para ayudar en lo que sea necesario. Si necesitas algo más, no dudes en decírmelo. Buena suerte con la guacamaya, y espero que todo salga bien" (`|MakeArray` "Continuar" :!type "Text")))
                  (switch `/Game/Blueprints/Enum_DialogueState` _state_4
                    (:`NewEnumerator0`
                      (`self.SetDialogueBranch` "BuscarJaula")
                      (`self.CloseConversation`))))))))))
    (:`BuscarJaula`
      (bind _state_5 (`self.AddDialogue` "Sarah" "Busca la jaula en la cancha de Basket"))
      (switch `/Game/Blueprints/Enum_DialogueState` _state_5
        (:`NewEnumerator0`
          (`self.ClearDialogueProgress`)
          (`self.CloseConversation`))))))