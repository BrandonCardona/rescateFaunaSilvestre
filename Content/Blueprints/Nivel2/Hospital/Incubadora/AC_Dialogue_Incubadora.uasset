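; Dialogue component for the hospital incubator in level 2, where the player character narrates in Spanish how the device works and watches an egg hatch.
; The default branch chains continue-only lines, then spawns an idle baby chicken at a fixed location, switches to the "incubadora" branch and closes the conversation.
; That branch shows a short line about more chicks hatching soon, then clears dialogue progress and closes.
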(fn `Dialogue`
  (`parent.Dialogue`)
  (switch `name` (`self.ActiveDialogueBranch`)
    (:`Default`
      (bind _state (`self.AddDialogue` "Tú" "Esta es la incubadora, uno de los dispositivos más importantes en el hospital de fauna silvestre. Aquí se cuidan los huevos y crías recién nacidas, manteniéndolas en un ambiente controlado y seguro" (`|MakeArray` "Continuar" :!type "Text")))
      (switch `/Game/Blueprints/Enum_DialogueState` _state
        (:`NewEnumerator0`
          (bind _state_2 (`self.AddDialogue` "Tú" "La incubadora simula las condiciones naturales que tendrían con sus madres, proporcionándoles el calor y la humedad necesarios para su desarrollo. Gracias a este aparato, podemos asegurar que los huevos reciban la temperatura adecuada y la humedad precisa para que el embrión se desarrolle correctamente" (`|MakeArray` "Continuar" :!type "Text")))
          (switch `/Game/Blueprints/Enum_DialogueState` _state_2
            (:`NewEnumerator0`
              (bind _state_3 (`self.AddDialogue` "Tú" "La incubadora también nos permite monitorear constantemente el progreso de los huevos y las crías. Con sus sensores y controles, podemos ajustar cualquier variable en tiempo real para garantizar el mejor entorno posible para estas pequeñas vidas" (`|MakeArray` "Continuar" :!type "Text")))
              (switch `/Game/Blueprints/Enum_DialogueState` _state_3
                (:`NewEnumerator0`
                  (bind _state_4 (`self.AddDialogue` "Tú" "Es fascinante pensar en la vida que se está gestando dentro de estos huevos" (`|MakeArray` "Continuar" :!type "Text")))
                  (switch `/Game/Blueprints/Enum_DialogueState` _state_4
                    (:`NewEnumerator0`
                      (bind _state_5 (`self.AddDialogue` "Tú" "¡Oh, espera un momento! Uno de los huevos está comenzando a moverse. Puedo ver una pequeña grieta formándose en la cáscara. Es increíble cómo la vida empieza de esta manera, con un pequeño ser luchando por salir al mundo" (`|MakeArray` "Continuar" :!type "Text")))
                      (switch `/Game/Blueprints/Enum_DialogueState` _state_5
                        (:`NewEnumerator0`
                          (bind _state_6 (`self.AddDialogue` "Tú" "La cáscara se está rompiendo más... ¡Ahí está! Un pequeño pico ha aparecido, y pronto, una cabecita mojada se asoma. Este polluelo es tan diminuto y frágil, pero lleno de potencial. Cada movimiento que hace para liberarse del huevo es un recordatorio de lo valioso que es este trabajo" (`|MakeArray` "Continuar" :!type "Text")))
                          (switch `/Game/Blueprints/Enum_DialogueState` _state_6
                            (:`NewEnumerator0`
                              (bind _state_7 (`self.AddDialogue` "Tú" "Finalmente, el polluelo ha salido por completo. Bienvenido al mundo, pequeño. Ahora empieza tu viaje, y aquí nos aseguraremos de que tengas el mejor comienzo posible" (`|MakeArray` "Continuar" :!type "Text")))
                              (switch `/Game/Blueprints/Enum_DialogueState` _state_7
                                (:`NewEnumerator0`
                                  (`|SpawnActorFromClass` "/Game/Blueprints/Animals/BabyChicken/BP_BabyChickenIdle.BP_BabyChickenIdle_C" (`KismetMathLibrary.MakeTransform` (585.0 -587.0 35.0)) "Undefined" "MultiplyWithRoot" null null)
                                  (`self.SetDialogueBranch` "incubadora")
                                  (`self.CloseConversation`))))))))))))))))
    (:`incubadora`
      (bind _state_8 (`self.AddDialogue` "Tú" "Pronto nacerán más pollos de la incubadora "))
      (switch `/Game/Blueprints/Enum_DialogueState` _state_8
        (:`NewEnumerator0`
          (`self.ClearDialogueProgress`)
          (`self.CloseConversation`))))))