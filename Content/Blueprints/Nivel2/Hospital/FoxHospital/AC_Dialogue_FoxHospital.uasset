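; Dialogue component for the hospital fox in Nivel2, where the player character ("Tú") muses on a red fox being treated at the CAV wildlife hospital.
; It overrides Dialogue, calls the parent and switches on the active dialogue branch.
; The default branch chains single-option lines on possible causes, care and conservation, then sets the "zorro" branch and closes.
; That branch gives a short line about awaiting quarantine or rehabilitation, clears dialogue progress and closes.
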(fn `Dialogue`
  (`parent.Dialogue`)
  (switch `name` (`self.ActiveDialogueBranch`)
    (:`Default`
      (bind _state (`self.AddDialogue` "Tú" "Ah, aquí tenemos a un zorro rojo, Vulpes vulpes. Este en particular está recibiendo tratamiento en el hospital del CAV" (`|MakeArray` "Continuar" :!type "Text")))
      (switch `/Game/Blueprints/Enum_DialogueState` _state
        (:`NewEnumerator0`
          (bind _state_2 (`self.AddDialogue` "Tú" "Los zorros son animales muy adaptables y suelen ser bastante resilientes, pero a veces incluso los depredadores enfrentan desafíos que los traen a estos centros" (`|MakeArray` "Continuar" :!type "Text")))
          (switch `/Game/Blueprints/Enum_DialogueState` _state_2
            (:`NewEnumerator0`
              (bind _state_3 (`self.AddDialogue` "Tú" "Podría estar aquí por varias razones. Tal vez sufrió alguna lesión debido a una trampa o un accidente vehicular, lo cual es bastante común en áreas donde los zorros cruzan carreteras frecuentemente" (`|MakeArray` "Continuar" :!type "Text")))
              (switch `/Game/Blueprints/Enum_DialogueState` _state_3
                (:`NewEnumerator0`
                  (bind _state_4 (`self.AddDialogue` "Tú" "También es posible que haya sido víctima de algún tipo de envenenamiento, ya sea por ingestión de sustancias tóxicas en su entorno o por consumir presas que han sido envenenadas" (`|MakeArray` "Continuar" :!type "Text")))
                  (switch `/Game/Blueprints/Enum_DialogueState` _state_4
                    (:`NewEnumerator0`
                      (bind _state_5 (`self.AddDialogue` "Tú" "Otro motivo podría ser una enfermedad. Los zorros son susceptibles a enfermedades como el moquillo o la rabia, que pueden debilitarlos significativamente" (`|MakeArray` "Continuar" :!type "Text")))
                      (switch `/Game/Blueprints/Enum_DialogueState` _state_5
                        (:`NewEnumerator0`
                          (bind _state_6 (`self.AddDialogue` "Tú" "Aquí en la sección de depredadores, se mantiene un ambiente controlado para que los animales puedan recuperarse sin estrés adicional. Asegurándose de que tengan un espacio seguro y cómodo, y los alimentamos con una dieta que les ayude a recuperarse rápidamente" (`|MakeArray` "Continuar" :!type "Text")))
                          (switch `/Game/Blueprints/Enum_DialogueState` _state_6
                            (:`NewEnumerator0`
                              (bind _state_7 (`self.AddDialogue` "Tú" "Es fascinante ver cómo estos animales, a pesar de ser depredadores, también necesitan de nuestra ayuda y cuidado en momentos de vulnerabilidad" (`|MakeArray` "Continuar" :!type "Text")))
                              (switch `/Game/Blueprints/Enum_DialogueState` _state_7
                                (:`NewEnumerator0`
                                  (bind _state_8 (`self.AddDialogue` "Tú" "Cada uno de ellos es vital para el equilibrio de nuestros ecosistemas, y mi trabajo como rescatista es crucial para asegurar su bienestar y conservación" (`|MakeArray` "Continuar" :!type "Text")))
                                  (switch `/Game/Blueprints/Enum_DialogueState` _state_8
                                    (:`NewEnumerator0`
                                      (`self.SetDialogueBranch` "zorro")
                                      (`self.CloseConversation`))))))))))))))))))
    (:`zorro`
      (bind _state_9 (`self.AddDialogue` "Tú" "Tendré que esperar para saber cuál será su destino. Si deberá ir a cuarentena o rehabilitación"))
      (switch `/Game/Blueprints/Enum_DialogueState` _state_9
        (:`NewEnumerator0`
          (`self.ClearDialogueProgress`)
          (`self.CloseConversation`))))))