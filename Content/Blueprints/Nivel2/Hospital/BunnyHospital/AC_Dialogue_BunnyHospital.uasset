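; Dialogue component for the hospital rabbit in level 2, where the player character narrates about a wild rabbit under treatment at the CAV.
; Overrides Dialogue, calling the parent, then switches on the active branch: the default chains educational lines on likely injuries, diseases and care through Continue options.
; That chain sets the "conejo" branch and closes the conversation.
; The Conejo branch shows a line about awaiting quarantine or rehabilitation, clears dialogue progress and closes.
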(fn `Dialogue`
  (`parent.Dialogue`)
  (switch `name` (`self.ActiveDialogueBranch`)
    (:`Default`
      (bind _state (`self.AddDialogue` "Tú" "Ah, aquí tenemos a un conejo silvestre, posiblemente un Oryctolagus cuniculus. Este pequeño está recibiendo tratamiento en el hospital del CAV" (`|MakeArray` "Continuar" :!type "Text")))
      (switch `/Game/Blueprints/Enum_DialogueState` _state
        (:`NewEnumerator0`
          (bind _state_2 (`self.AddDialogue` "Tú" "Los conejos son animales muy sensibles y pueden verse afectados por diversos factores que los llevan a necesitar nuestra ayuda. Este en particular podría haber sido víctima de un ataque de un depredador, ya que los conejos son presas comunes para muchos carnívoros" (`|MakeArray` "Continuar" :!type "Text")))
          (switch `/Game/Blueprints/Enum_DialogueState` _state_2
            (:`NewEnumerator0`
              (bind _state_3 (`self.AddDialogue` "Tú" "Otra posibilidad es que haya sido herido en una trampa o haya sufrido una lesión accidental mientras buscaba comida. Los conejos también son propensos a ciertas enfermedades como la mixomatosis o la enfermedad hemorrágica viral, que pueden debilitarlos gravemente y requieren atención médica especializada" (`|MakeArray` "Continuar" :!type "Text")))
              (switch `/Game/Blueprints/Enum_DialogueState` _state_3
                (:`NewEnumerator0`
                  (bind _state_4 (`self.AddDialogue` "Tú" "En esta sección del hospital, se aseguran de que los conejos y otros animales presa tengan un ambiente tranquilo y seguro para su recuperación" (`|MakeArray` "Continuar" :!type "Text")))
                  (switch `/Game/Blueprints/Enum_DialogueState` _state_4
                    (:`NewEnumerator0`
                      (bind _state_5 (`self.AddDialogue` "Tú" "Es sorprendente ver cuánta resiliencia tienen estos pequeños animales y lo importante que es nuestra intervención para su recuperación. Cada conejo que se cuida aquí es un recordatorio de la delicada interacción entre las especies y nuestro papel en la conservación de la vida silvestre" (`|MakeArray` "Continuar" :!type "Text")))
                      (switch `/Game/Blueprints/Enum_DialogueState` _state_5
                        (:`NewEnumerator0`
                          (`self.SetDialogueBranch` "conejo")
                          (`self.CloseConversation`))))))))))))
    (:`conejo`
      (bind _state_6 (`self.AddDialogue` "Tú" "Tendré que esperar para saber cuál será su destino. Si deberá ir a cuarentena o rehabilitación"))
      (switch `/Game/Blueprints/Enum_DialogueState` _state_6
        (:`NewEnumerator0`
          (`self.ClearDialogueProgress`)
          (`self.CloseConversation`))))))