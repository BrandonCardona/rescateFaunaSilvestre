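; Dialogue component for Daniela at the CAV bioterio in Nivel2, where she explains in Spanish how feeder animals are bred for the predators in care.
; The Dialogue graph calls its parent, then switches on the active branch.
; The default branch chains Continuar prompts through her explanation, then sets the Bioterio branch and closes the conversation.
; The Bioterio branch directs the player to explore and head to quarantine, then clears dialogue progress and closes.
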(fn `Dialogue`
  (`parent.Dialogue`)
  (switch `name` (`self.ActiveDialogueBranch`)
    (:`Default`
      (bind _state (`self.AddDialogue` "Daniela" "¡Hola de nuevo, rescatista! Bienvenido al bioterio del CAV. Este es un lugar crucial para el cuidado y nutrición de muchos de los animales que tenemos aquí" (`|MakeArray` "Continuar" :!type "Text")))
      (switch `/Game/Blueprints/Enum_DialogueState` _state
        (:`NewEnumerator0`
          (bind _state_2 (`self.AddDialogue` "Daniela" "El bioterio es donde criamos y mantenemos a los animales que se utilizarán como alimento para nuestros depredadores. Aquí criamos conejos, ratones y cucarachas, asegurándonos de que estén en condiciones óptimas de salud y nutrición para proporcionar una dieta balanceada y natural a nuestros animales carnívoros" (`|MakeArray` "Continuar" :!type "Text")))
          (switch `/Game/Blueprints/Enum_DialogueState` _state_2
            (:`NewEnumerator0`
              (bind _state_3 (`self.AddDialogue` "Daniela" "En primer lugar, déjame explicarte por qué es tan importante el bioterio. Muchos de los depredadores que atendemos en el hospital necesitan una dieta específica para recuperarse y mantener su salud. Proveerles alimentos vivos o recién sacrificados les permite tener una alimentación que se asemeja a lo que encontrarían en la naturaleza, lo que es esencial para su bienestar físico y psicológico" (`|MakeArray` "Continuar" :!type "Text")))
              (switch `/Game/Blueprints/Enum_DialogueState` _state_3
                (:`NewEnumerator0`
                  (bind _state_4 (`self.AddDialogue` "Daniela" "Criar nuestros propios animales de alimentación nos asegura el control de calidad en todos los aspectos. Podemos controlar su dieta, su salud y sus condiciones de vida, garantizando que sean una fuente de alimento segura y nutritiva para nuestros depredadores. Además, esto nos ayuda a prevenir la introducción de enfermedades y parásitos que podrían venir con animales adquiridos de fuentes externas" (`|MakeArray` "Continuar" :!type "Text")))
                  (switch `/Game/Blueprints/Enum_DialogueState` _state_4
                    (:`NewEnumerator0`
                      (bind _state_5 (`self.AddDialogue` "Daniela" "Además, mantenemos estrictas medidas de bioseguridad en el bioterio. Esto incluye controles sanitarios regulares, un ambiente controlado y protocolos de manejo para minimizar el riesgo de enfermedades. Todo esto es fundamental para asegurar que tanto los animales de alimentación como nuestros depredadores se mantengan saludables" (`|MakeArray` "Continuar" :!type "Text")))
                      (switch `/Game/Blueprints/Enum_DialogueState` _state_5
                        (:`NewEnumerator0`
                          (bind _state_6 (`self.AddDialogue` "Daniela" "Espero que esta visita al bioterio te dé una mejor comprensión de la importancia de esta área en el cuidado y rehabilitación de la fauna silvestre. Gracias por tu dedicación y por ser parte de nuestro equipo de rescate. ¡Sigamos trabajando juntos para proteger y cuidar a la fauna silvestre!" (`|MakeArray` "Continuar" :!type "Text")))
                          (switch `/Game/Blueprints/Enum_DialogueState` _state_6
                            (:`NewEnumerator0`
                              (bind _state_7 (`self.AddDialogue` "Daniela" "En el área de depredadores, atendemos a animales como zorros, aves rapaces y otros carnívoros que requieren un manejo y tratamiento especial. Nos aseguramos de que estos animales tengan un espacio adecuado donde puedan recuperarse sin el riesgo de estresar a los animales presa" (`|MakeArray` "Continuar" :!type "Text")))
                              (switch `/Game/Blueprints/Enum_DialogueState` _state_7
                                (:`NewEnumerator0`
                                  (bind _state_8 (`self.AddDialogue` "Daniela" "¡Ahora, te invito a seguirme para mostrarte las instalaciones del bioterio y que puedas ver todo esto en detalle!" (`|MakeArray` "Continuar" :!type "Text")))
                                  (switch `/Game/Blueprints/Enum_DialogueState` _state_8
                                    (:`NewEnumerator0`
                                      (`self.SetDialogueBranch` "Bioterio")
                                      (`self.CloseConversation`))))))))))))))))))
    (:`Bioterio`
      (bind _state_9 (`self.AddDialogue` "Daniela" "Explora el hospital por tu cuenta y luego dirígete a la zona de cuarentena "))
      (switch `/Game/Blueprints/Enum_DialogueState` _state_9
        (:`NewEnumerator0`
          (`self.ClearDialogueProgress`)
          (`self.CloseConversation`))))))