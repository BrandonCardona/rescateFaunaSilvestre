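; Dialogue component for the hedgehog in the level 2 clinic, where the player's character shares facts about the European hedgehog and its likely evaluation.
; It overrides Dialogue, calling the parent, then switches on the active branch.
; The default branch chains monologue lines, then sets the "erizo" branch and closes the conversation.
; That branch shows a line about awaiting quarantine, hospital or rehabilitation, then clears progress and closes.
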(fn `Dialogue`
  (`parent.Dialogue`)
  (switch `name` (`self.ActiveDialogueBranch`)
    (:`Default`
      (bind _state (`self.AddDialogue` "Tú" "¡Oh, mira quién está aquí! Este es un erizo común europeo, científicamente conocido como Erinaceus europaeus. Son criaturas fascinantes" (`|MakeArray` "Continuar" :!type "Text")))
      (switch `/Game/Blueprints/Enum_DialogueState` _state
        (:`NewEnumerator0`
          (bind _state_2 (`self.AddDialogue` "Tú" "Es sorprendente saber que los erizos tienen alrededor de 5000 púas en su cuerpo, y cada una de ellas es hueca y actúa como un tubo de aire, lo que les permite flotar en el agua. Además, son excelentes nadadores y trepadores, a pesar de su apariencia un poco torpe" (`|MakeArray` "Continuar" :!type "Text")))
          (switch `/Game/Blueprints/Enum_DialogueState` _state_2
            (:`NewEnumerator0`
              (bind _state_3 (`self.AddDialogue` "Tú" "Ahora, con respecto a su evaluación aquí en el consultorio, puedo suponer que probablemente esté siendo revisado principalmente en la parte clínica debido a una lesión o herida" (`|MakeArray` "Continuar" :!type "Text")))
              (switch `/Game/Blueprints/Enum_DialogueState` _state_3
                (:`NewEnumerator0`
                  (bind _state_4 (`self.AddDialogue` "Tú" "Los erizos son animales bastante curiosos y pueden meterse en problemas, especialmente si se topan con objetos extraños o peligrosos en su entorno" (`|MakeArray` "Continuar" :!type "Text")))
                  (switch `/Game/Blueprints/Enum_DialogueState` _state_4
                    (:`NewEnumerator0`
                      (bind _state_5 (`self.AddDialogue` "Tú" "Sin embargo, también es posible que estemos evaluando su estado nutricional, ya que una dieta inadecuada puede afectar su salud en general" (`|MakeArray` "Continuar" :!type "Text")))
                      (switch `/Game/Blueprints/Enum_DialogueState` _state_5
                        (:`NewEnumerator0`
                          (bind _state_6 (`self.AddDialogue` "Tú" "Los erizos son omnívoros y necesitan una dieta variada que incluya insectos, frutas, verduras y proteínas para mantenerse saludables" (`|MakeArray` "Continuar" :!type "Text")))
                          (switch `/Game/Blueprints/Enum_DialogueState` _state_6
                            (:`NewEnumerator1`
                              (`self.SetDialogueBranch` "erizo")
                              (`self.CloseConversation`))))))))))))))
    (:`erizo`
      (bind _state_7 (`self.AddDialogue` "Tú" "Tendré que esperar para saber cual será su destino. Si deberá ir a cuarentena, hospital o rehabilitación"))
      (switch `/Game/Blueprints/Enum_DialogueState` _state_7
        (:`NewEnumerator0`
          (`self.ClearDialogueProgress`)
          (`self.CloseConversation`))))))