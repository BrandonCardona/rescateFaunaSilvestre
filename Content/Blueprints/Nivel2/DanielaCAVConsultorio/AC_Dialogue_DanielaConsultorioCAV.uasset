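; Dialogue component for Daniela, who welcomes the player to a wildlife care and assessment center (CAV) and introduces its consultation room in Spanish.
; It overrides Dialogue, calls the parent, then switches on the active branch.
; The default branch chains "Continuar" lines on clinical, biological and nutritional evaluation, then sets the Consultorio branch and closes.
; That branch tells the player to explore the cages and head to the hospital, then clears progress and closes.
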(fn `Dialogue`
  (`parent.Dialogue`)
  (switch `name` (`self.ActiveDialogueBranch`)
    (:`Default`
      (bind _state (`self.AddDialogue` "Daniela" "¡Hola y bienvenido al Centro de Atención y Valoración de Fauna Silvestre! Soy Daniela, encargada de recibir a nuestros valiosos rescatistas como tú. Estoy emocionada de tenerte aquí y de compartir contigo un poco sobre lo que hacemos en nuestro centro" (`|MakeArray` "Continuar" :!type "Text")))
      (switch `/Game/Blueprints/Enum_DialogueState` _state
        (:`NewEnumerator0`
          (bind _state_2 (`self.AddDialogue` "Daniela" "En primer lugar, tenemos el consultorio. Aquí llegan todos los animales en primer lugar" (`|MakeArray` "Continuar" :!type "Text")))
          (switch `/Game/Blueprints/Enum_DialogueState` _state_2
            (:`NewEnumerator0`
              (bind _state_3 (`self.AddDialogue` "Daniela" "En esta área, nos enfocamos en tres aspectos principales: clínico, biológico y nutricional" (`|MakeArray` "Continuar" :!type "Text")))
              (switch `/Game/Blueprints/Enum_DialogueState` _state_3
                (:`NewEnumerator0`
                  (bind _state_4 (`self.AddDialogue` "Daniela" "Empecemos por la parte clínica. Aquí evaluamos cualquier herida o condición médica que pueda tener el animal rescatado. Es crucial asegurarnos de que estén en óptimas condiciones de salud para proceder con su rehabilitación o liberación" (`|MakeArray` "Continuar" :!type "Text")))
                  (switch `/Game/Blueprints/Enum_DialogueState` _state_4
                    (:`NewEnumerator0`
                      (bind _state_5 (`self.AddDialogue` "Daniela" "Luego está la parte biológica, donde estudiamos las características del animal, como su comportamiento, medidas, edad y cualquier otra información relevante que nos ayude a comprender mejor sus necesidades y estado general" (`|MakeArray` "Continuar" :!type "Text")))
                      (switch `/Game/Blueprints/Enum_DialogueState` _state_5
                        (:`NewEnumerator0`
                          (bind _state_6 (`self.AddDialogue` "Daniela" "Y por último, pero no menos importante, está la parte nutricional. Donde nos aseguramos de que el animal esté recibiendo la alimentación adecuada para su recuperación. Esto incluye evaluar su peso, músculos, huesos y su capacidad para alimentarse correctamente" (`|MakeArray` "Continuar" :!type "Text")))
                          (switch `/Game/Blueprints/Enum_DialogueState` _state_6
                            (:`NewEnumerator0`
                              (bind _state_7 (`self.AddDialogue` "Daniela" "Una vez que hemos recopilado toda esta información, podemos determinar si el animal necesita ser puesto en cuarentena, pasar por un proceso de rehabilitación, ser tratado en el hospital o estar listo para ser liberado de nuevo en su hábitat natural" (`|MakeArray` "Continuar" :!type "Text")))
                              (switch `/Game/Blueprints/Enum_DialogueState` _state_7
                                (:`NewEnumerator0`
                                  (bind _state_8 (`self.AddDialogue` "Daniela" "¡Ahora, te invito a seguirme para mostrarte las jaulas donde tenemos a los animales que están siendo evaluados en este momento!" (`|MakeArray` "Continuar" :!type "Text")))
                                  (switch `/Game/Blueprints/Enum_DialogueState` _state_8
                                    (:`NewEnumerator0`
                                      (`self.SetDialogueBranch` "Consultorio")
                                      (`self.CloseConversation`))))))))))))))))))
    (:`Consultorio`
      (bind _state_9 (`self.AddDialogue` "Daniela" "Explora las jaulas por tu cuenta y luego dirígete al hospital "))
      (switch `/Game/Blueprints/Enum_DialogueState` _state_9
        (:`NewEnumerator0`
          (`self.ClearDialogueProgress`)
          (`self.CloseConversation`))))))