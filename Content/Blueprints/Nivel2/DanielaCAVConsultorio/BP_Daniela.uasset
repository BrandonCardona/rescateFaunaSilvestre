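; BP_Daniela is a flipbook-animated character, Daniela, that walks a short scripted path in the Nivel2 consultorio area.
; Ending overlap with Box starts her walking right, with Tick feeding forward movement input while Mover is set.
; The first WalkDetector overlap rotates her and swaps to the up-walk flipbook.
; Contador makes later overlaps rotate her again, show the idle-down flipbook and stop movement.
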(event `self.ReceiveTick`
  (params (DeltaSeconds :type "Float (single-precision)"))
  (if (`self.mover`)
    (`self.AddMovementInput` (`self.GetActorForwardVector`))))

(event `self.WalkDetector.OnComponentBeginOverlap`
  (params (OverlappedComponent :type "PrimitiveComponent Object Reference") (OtherActor :type "Actor Object Reference") (OtherComp :type "PrimitiveComponent Object Reference") (OtherBodyIndex :type Integer) (bFromSweep :type Boolean) (SweepResult :type "HitResult Structure (by ref)"))
  (if (< (`self.contador`) 1)
    (`self.TurnChar`)
    (bind _result (`/Engine/EditorBlueprintResources/StandardMacros.IncrementInt` (`self.contador`))
      (:`  `
        (set `self.contador` _result)))
    (else
      (`self.Reposo`)
      (set `self.mover` false))))

(event `self.Box.OnComponentEndOverlap`
  (params (OverlappedComponent :type "PrimitiveComponent Object Reference") (OtherActor :type "Actor Object Reference") (OtherComp :type "PrimitiveComponent Object Reference") (OtherBodyIndex :type Integer))
  (if (< (`self.contador`) 1)
    (`PaperFlipbookComponent.SetFlipbook` (`self.Sprite`) "/Game/Assets/NPCPersons/Daniela/Right/Daniela_Right.Daniela_Right")
    (set `self.mover` true)))

(fn `Reposo`
  (`self.K2_SetActorRotation` (`KismetMathLibrary.ComposeRotators` (`self.K2_GetActorRotation`) (struct :`Yaw` 90.0)))
  (`PaperFlipbookComponent.SetFlipbook` (`self.Sprite`) "/Game/Assets/NPCPersons/Daniela/IdleDown/Daniela_IdleDown.Daniela_IdleDown"))

(fn `TurnChar`
  (`self.K2_SetActorRotation` (`KismetMathLibrary.ComposeRotators` (`self.K2_GetActorRotation`) (struct :`Yaw` 270.0)))
  (`PaperFlipbookComponent.SetFlipbook` (`self.Sprite`) "/Game/Assets/NPCPersons/Daniela/UpReverse/Daniela_UpReverse.Daniela_UpReverse"))

(fn `UserConstructionScript`)