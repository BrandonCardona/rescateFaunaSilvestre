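; Dialogue component for Daniela, the NPC in Level 2's wildlife center quarantine zone, who explains quarantine care and assigns the turtle-feeding task.
; It overrides Dialogue and switches on the active branch, chaining AddDialogue lines through their Pass Through state.
; The default branch plays the introduction, then sets the "Cuarentena" branch and closes the conversation.
; That branch repeats the feeding reminder, clears dialogue progress and closes.
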(fn `Dialogue`
  (`parent.Dialogue`)
  (switch `name` (`self.ActiveDialogueBranch`)
    (:`Default`
      (bind _state (`self.AddDialogue` "Daniela" "Bienvenido a la zona de cuarentena del Centro de Atención y Valoración de Fauna Silvestre. Esta área es esencial para el cuidado de los animales que han sido lastimados o aquellos cuyo comportamiento ha sido afectado debido a su contacto con humanos" (`|MakeArray` "Continuar" :!type "Text")))
      (switch `/Game/Blueprints/Enum_DialogueState` _state
        (:`NewEnumerator0`
          (bind _state_2 (`self.AddDialogue` "Daniela" "En la zona de cuarentena, mantenemos a los animales en jaulas individuales y en un ambiente controlado. Esto nos permite observar y tratar a los animales heridos, así como darles el espacio necesario para que puedan volver a comportarse de manera natural, sin la influencia del contacto humano. Es crucial que minimicemos nuestra interacción directa con ellos para ayudarles a recuperar su comportamiento instintivo y natural" (`|MakeArray` "Continuar" :!type "Text")))
          (switch `/Game/Blueprints/Enum_DialogueState` _state_2
            (:`NewEnumerator0`
              (bind _state_3 (`self.AddDialogue` "Daniela" "Las jaulas aquí son sometidas a una limpieza exhaustiva regularmente. Esto garantiza un entorno higiénico y seguro, reduciendo el riesgo de infecciones y facilitando una recuperación más rápida y efectiva para los animales" (`|MakeArray` "Continuar" :!type "Text")))
              (switch `/Game/Blueprints/Enum_DialogueState` _state_3
                (:`NewEnumerator0`
                  (bind _state_4 (`self.AddDialogue` "Daniela" "Nuestro equipo especializado monitorea de cerca a cada animal, asegurándose de que reciban los cuidados médicos y la observación necesaria hasta que estén listos para ser trasladados a otras áreas del centro como la zona de rehabilitación" (`|MakeArray` "Continuar" :!type "Text")))
                  (switch `/Game/Blueprints/Enum_DialogueState` _state_4
                    (:`NewEnumerator0`
                      (bind _state_5 (`self.AddDialogue` "Daniela" "Ahora, necesitamos alimentar a una de nuestras tortugas que se encuentra en cuarentena. Por favor, dirígete al área de almacenamiento de alimentos y busca la comida especial para tortugas. Es crucial que sigamos una dieta específica para cada especie, asegurándonos de que reciben todos los nutrientes que necesitan para su recuperación" (`|MakeArray` "Continuar" :!type "Text")))
                      (switch `/Game/Blueprints/Enum_DialogueState` _state_5
                        (:`NewEnumerator0`
                          (bind _state_6 (`self.AddDialogue` "Daniela" "Gracias por tu ayuda y dedicación. Cada pequeño esfuerzo cuenta en nuestra misión de cuidar y rehabilitar a la fauna silvestre" (`|MakeArray` "Continuar" :!type "Text")))
                          (switch `/Game/Blueprints/Enum_DialogueState` _state_6
                            (:`NewEnumerator0`
                              (`self.SetDialogueBranch` "Cuarentena")
                              (`self.CloseConversation`))))))))))))))
    (:`Cuarentena`
      (bind _state_7 (`self.AddDialogue` "Daniela" "Busca el alimento de la tortuga en el almacén y aliméntala"))
      (switch `/Game/Blueprints/Enum_DialogueState` _state_7
        (:`NewEnumerator0`
          (`self.ClearDialogueProgress`)
          (`self.CloseConversation`))))))