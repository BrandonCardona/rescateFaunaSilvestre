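; Dialogue component for the NPC Daniela in Nivel2 that sends the player to the rehabilitation zone after they help feed the turtle.
; It extends the parent Dialogue and switches on the active branch, stepping through lines as each passes through.
; The default branch plays the thanks and directions, then switches to the "Cuarentena" branch, which repeats a short reminder and clears dialogue progress before closing.
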(fn `Dialogue`
  (`parent.Dialogue`)
  (switch `name` (`self.ActiveDialogueBranch`)
    (:`Default`
      (bind _state (`self.AddDialogue` "Daniela" "Agradezco mucho tu ayuda alimentando a la tortuga"))
      (switch `/Game/Blueprints/Enum_DialogueState` _state
        (:`NewEnumerator0`
          (bind _state_2 (`self.AddDialogue` "Daniela" " Ahora debes dirigir a la zona de rehabilitación "))
          (switch `/Game/Blueprints/Enum_DialogueState` _state_2
            (:`NewEnumerator0`
              (`self.SetDialogueBranch` "Cuarentena")
              (`self.CloseConversation`))))))
    (:`Cuarentena`
      (bind _state_3 (`self.AddDialogue` "Daniela" "Ve a la zona de rehabilitación "))
      (switch `/Game/Blueprints/Enum_DialogueState` _state_3
        (:`NewEnumerator0`
          (`self.ClearDialogueProgress`)
          (`self.CloseConversation`))))))