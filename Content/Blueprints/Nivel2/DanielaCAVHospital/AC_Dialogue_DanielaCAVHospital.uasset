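; Dialogue component for Daniela, the NPC who introduces the wildlife rescue center's (CAV) hospital area in level 2, with Spanish text.
; It overrides Dialogue, calls the parent, then switches on the active dialogue branch.
; The default branch chains Continue-only lines about incubation, prey and predator wards and animal groups, then switches to the Hospital branch.
; That branch tells the player to explore and head to the bioterium, then clears progress and closes.
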(fn `Dialogue`
  (`parent.Dialogue`)
  (switch `name` (`self.ActiveDialogueBranch`)
    (:`Default`
      (bind _state (`self.AddDialogue` "Daniela" "¡Hola de nuevo, rescatista! Bienvenido a la zona del hospital del Centro de Atención y Valoración de Fauna Silvestre. Aquí es donde brindamos el cuidado intensivo y especializado que muchos de nuestros animales necesitan para su recuperación" (`|MakeArray` "Continuar" :!type "Text")))
      (switch `/Game/Blueprints/Enum_DialogueState` _state
        (:`NewEnumerator0`
          (bind _state_2 (`self.AddDialogue` "Daniela" "En el hospital, tenemos varias áreas dedicadas a diferentes tipos de tratamiento y cuidados médicos" (`|MakeArray` "Continuar" :!type "Text")))
          (switch `/Game/Blueprints/Enum_DialogueState` _state_2
            (:`NewEnumerator0`
              (bind _state_3 (`self.AddDialogue` "Daniela" "En primer lugar está el área de incubación, donde tenemos una incubadora especial donde cuidamos a los pollos y otras aves jóvenes que necesitan un ambiente controlado para sobrevivir y prosperar" (`|MakeArray` "Continuar" :!type "Text")))
              (switch `/Game/Blueprints/Enum_DialogueState` _state_3
                (:`NewEnumerator0`
                  (bind _state_4 (`self.AddDialogue` "Daniela" "La incubadora mantiene la temperatura y la humedad adecuadas, cruciales para la salud y el desarrollo de los polluelos. Además, monitoreamos de cerca su crecimiento y los alimentamos con una dieta balanceada para asegurarnos de que reciban todos los nutrientes necesarios" (`|MakeArray` "Continuar" :!type "Text")))
                  (switch `/Game/Blueprints/Enum_DialogueState` _state_4
                    (:`NewEnumerator0`
                      (bind _state_5 (`self.AddDialogue` "Daniela" "Luego, para garantizar la seguridad y el bienestar de todos los animales, hemos dividido nuestra zona de hospitalización en dos áreas separadas: una para animales presa y otra para animales depredadores" (`|MakeArray` "Continuar" :!type "Text")))
                      (switch `/Game/Blueprints/Enum_DialogueState` _state_5
                        (:`NewEnumerator0`
                          (bind _state_6 (`self.AddDialogue` "Daniela" "En el área de animales presa cuidamos de animales como conejos, aves pequeñas y roedores que necesitan atención médica. Este área está diseñada para proporcionar un entorno tranquilo y seguro, lejos de cualquier estrés que pudiera ser causado por la presencia de depredadores" (`|MakeArray` "Continuar" :!type "Text")))
                          (switch `/Game/Blueprints/Enum_DialogueState` _state_6
                            (:`NewEnumerator0`
                              (bind _state_7 (`self.AddDialogue` "Daniela" "En el área de depredadores, atendemos a animales como zorros, aves rapaces y otros carnívoros que requieren un manejo y tratamiento especial. Nos aseguramos de que estos animales tengan un espacio adecuado donde puedan recuperarse sin el riesgo de estresar a los animales presa" (`|MakeArray` "Continuar" :!type "Text")))
                              (switch `/Game/Blueprints/Enum_DialogueState` _state_7
                                (:`NewEnumerator0`
                                  (bind _state_8 (`self.AddDialogue` "Daniela" "Además, para organizar mejor nuestros cuidados y tratamientos, hemos dividido los animales en tres grupos principales: aves, mamíferos y reptiles" (`|MakeArray` "Continuar" :!type "Text")))
                                  (switch `/Game/Blueprints/Enum_DialogueState` _state_8
                                    (:`NewEnumerator0`
                                      (bind _state_9 (`self.AddDialogue` "Daniela" "Cada grupo tiene sus propias necesidades y requerimientos específicos, por lo que esta división nos ayuda a brindar una atención más eficaz y especializada" (`|MakeArray` "Continuar" :!type "Text")))
                                      (switch `/Game/Blueprints/Enum_DialogueState` _state_9
                                        (:`NewEnumerator0`
                                          (bind _state_10 (`self.AddDialogue` "Daniela" "Estoy segura de que esta visita al hospital te dará una mejor comprensión de la importancia y el alcance del trabajo que realizamos aquí. Gracias por tu dedicación y por ser parte de nuestro equipo de rescate. ¡Sigamos trabajando juntos para proteger y cuidar a la fauna silvestre!" (`|MakeArray` "Continuar" :!type "Text")))
                                          (switch `/Game/Blueprints/Enum_DialogueState` _state_10
                                            (:`NewEnumerator0`
                                              (bind _state_11 (`self.AddDialogue` "Daniela" "¡Ahora, te invito a seguirme para mostrarte el hospital y puedas verlo todo con un mayor detalle!" (`|MakeArray` "Continuar" :!type "Text")))
                                              (switch `/Game/Blueprints/Enum_DialogueState` _state_11
                                                (:`NewEnumerator0`
                                                  (`self.SetDialogueBranch` "Hospital")
                                                  (`self.CloseConversation`))))))))))))))))))))))))
    (:`Hospital`
      (bind _state_12 (`self.AddDialogue` "Daniela" "Explora el hospital por tu cuenta y luego dirígete al bioterio "))
      (switch `/Game/Blueprints/Enum_DialogueState` _state_12
        (:`NewEnumerator0`
          (`self.ClearDialogueProgress`)
          (`self.CloseConversation`))))))