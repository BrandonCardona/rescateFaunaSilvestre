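; Dialogue component for the quarantine area of level 2: the player's Spanish monologue before feeding, about a tortoise despite the Parrot naming.
; The default branch chains four lines on the animal and food placement, spawns NPC_FoodParrot at a hardcoded location, switches to the "Buscar" branch and closes.
; The "Buscar" branch shows a reminder to find a feeding spot, then clears dialogue progress and closes the conversation.
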(fn `Dialogue`
  (`parent.Dialogue`)
  (switch `name` (`self.ActiveDialogueBranch`)
    (:`Default`
      (bind _state (`self.AddDialogue` "Tú" "¡Ah, aquí está nuestra tortuga en cuarentena! Esta es una tortuga de piel verde y caparazón marrón, científicamente conocida como Testudo hermanni." (`|MakeArray` "Continuar" :!type "Text")))
      (switch `/Game/Blueprints/Enum_DialogueState` _state
        (:`NewEnumerator0`
          (bind _state_2 (`self.AddDialogue` "Tú" "Es interesante saber que estas tortugas pueden vivir hasta 50 años o más en condiciones adecuadas y tienen una increíble capacidad para recordar rutas y lugares de alimentación" (`|MakeArray` "Continuar" :!type "Text")))
          (switch `/Game/Blueprints/Enum_DialogueState` _state_2
            (:`NewEnumerator0`
              (bind _state_3 (`self.AddDialogue` "Tú" "Ahora, necesito encontrar un lugar adecuado para colocar la comida. Es importante que esté en un área donde la tortuga pueda acceder fácilmente, pero que también esté limpia y segurapsicológico" (`|MakeArray` "Continuar" :!type "Text")))
              (switch `/Game/Blueprints/Enum_DialogueState` _state_3
                (:`NewEnumerator0`
                  (bind _state_4 (`self.AddDialogue` "Tú" "Dado que las tortugas a menudo prefieren comer en el agua, colocaré los trozos de manzana cerca del borde del estanque" (`|MakeArray` "Continuar" :!type "Text")))
                  (switch `/Game/Blueprints/Enum_DialogueState` _state_4
                    (:`NewEnumerator0`
                      (`|SpawnActorFromClass` "/Game/Blueprints/Nivel2/Cuarentena/Parrot/Food/NPC_FoodParrot.NPC_FoodParrot_C" (`KismetMathLibrary.MakeTransform` (2329.0 -379.0 20.0)) "AlwaysSpawn" "MultiplyWithRoot" null null)
                      (`self.SetDialogueBranch` "Buscar")
                      (`self.CloseConversation`))))))))))
    (:`Buscar`
      (bind _state_5 (`self.AddDialogue` "Tú" "Debo buscar un lugar para colocar la comida de la tortuga"))
      (switch `/Game/Blueprints/Enum_DialogueState` _state_5
        (:`NewEnumerator0`
          (`self.ClearDialogueProgress`)
          (`self.CloseConversation`))))))