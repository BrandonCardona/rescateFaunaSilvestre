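; Dialogue component for the mouse-breeding sign in the Level 2 vivarium, presenting Spanish educational text spoken by "Letrero".
; It overrides the Dialogue function, calls the parent, then branches on the active dialogue branch.
; The default branch chains lines explaining how mice feed the wildlife center's recovering predators, then switches to the "Mouse" branch and closes.
; That branch shows a short reminder line, clears dialogue progress and closes the conversation.
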(fn `Dialogue`
  (`parent.Dialogue`)
  (switch `name` (`self.ActiveDialogueBranch`)
    (:`Default`
      (bind _state (`self.AddDialogue` "Letrero" "Zona de cría de ratones del Centro de Atención y Valoración de Fauna Silvestre" (`|MakeArray` "Continuar" :!type "Text")))
      (switch `/Game/Blueprints/Enum_DialogueState` _state
        (:`NewEnumerator0`
          (bind _state_2 (`self.AddDialogue` "Letrero" "Se crían ratones de manera controlada y segura para asegurar una fuente de alimento saludable y nutritiva para los depredadores" (`|MakeArray` "Continuar" :!type "Text")))
          (switch `/Game/Blueprints/Enum_DialogueState` _state_2
            (:`NewEnumerator0`
              (bind _state_3 (`self.AddDialogue` "Letrero" "Los ratones son una parte esencial de la dieta de varios depredadores que se cuidan en el centro" (`|MakeArray` "Continuar" :!type "Text")))
              (switch `/Game/Blueprints/Enum_DialogueState` _state_3
                (:`NewEnumerator0`
                  (bind _state_4 (`self.AddDialogue` "Letrero" "Entre ellos se encuentran las aves rapaces como halcones, búhos y águilas, los reptiles como serpientes y lagartos grandes y los mamíferos carnívoros como zorros y pequeños felinos" (`|MakeArray` "Continuar" :!type "Text")))
                  (switch `/Game/Blueprints/Enum_DialogueState` _state_4
                    (:`NewEnumerator0`
                      (bind _state_5 (`self.AddDialogue` "Letrero" "Nuestra prioridad es mantener a los ratones en condiciones óptimas de salud y bienestar. Así, se garantiza que proporcionen la mejor nutrición posible a los depredadores que dependen de ellos para su recuperación y supervivencia" (`|MakeArray` "Continuar" :!type "Text")))
                      (switch `/Game/Blueprints/Enum_DialogueState` _state_5
                        (:`NewEnumerator0`
                          (bind _state_6 (`self.AddDialogue` "Letrero" "Gracias por tu interés y por contribuir a la conservación de la vida silvestre" (`|MakeArray` "Continuar" :!type "Text")))
                          (switch `/Game/Blueprints/Enum_DialogueState` _state_6
                            (:`NewEnumerator0`
                              (`self.SetDialogueBranch` "Mouse")
                              (`self.CloseConversation`))))))))))))))
    (:`Mouse`
      (bind _state_7 (`self.AddDialogue` "Letrero" "Aquí se crían los ratones "))
      (switch `/Game/Blueprints/Enum_DialogueState` _state_7
        (:`NewEnumerator0`
          (`self.ClearDialogueProgress`)
          (`self.CloseConversation`))))))