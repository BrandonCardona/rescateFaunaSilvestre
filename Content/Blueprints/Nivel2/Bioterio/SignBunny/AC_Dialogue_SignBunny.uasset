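; Dialogue component for the rabbit-breeding sign in the Nivel2 Bioterio, spoken in Spanish as "Letrero".
; It overrides Dialogue, calls the parent, then switches on the active dialogue branch.
; The default branch chains six educational lines on rabbits bred as food for rescued predators, then sets the "Bunny" branch and closes the conversation.
; The Bunny branch shows a short reminder line, clears dialogue progress and closes.
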(fn `Dialogue`
  (`parent.Dialogue`)
  (switch `name` (`self.ActiveDialogueBranch`)
    (:`Default`
      (bind _state (`self.AddDialogue` "Letrero" "Zona de cría de conejos del Centro de Atención y Valoración de Fauna Silvestre" (`|MakeArray` "Continuar" :!type "Text")))
      (switch `/Game/Blueprints/Enum_DialogueState` _state
        (:`NewEnumerator0`
          (bind _state_2 (`self.AddDialogue` "Letrero" "En esta área, se crían conejos de manera controlada y ética para asegurar una fuente de alimento saludable y nutritiva para nuestros depredadores" (`|MakeArray` "Continuar" :!type "Text")))
          (switch `/Game/Blueprints/Enum_DialogueState` _state_2
            (:`NewEnumerator0`
              (bind _state_3 (`self.AddDialogue` "Letrero" "Los conejos son una parte crucial de la dieta de varios depredadores que cuidamos en el centro" (`|MakeArray` "Continuar" :!type "Text")))
              (switch `/Game/Blueprints/Enum_DialogueState` _state_3
                (:`NewEnumerator0`
                  (bind _state_4 (`self.AddDialogue` "Letrero" "Entre ellos se encuentran las aves rapaces como águilas, búhos y halcones, los mamíferos carnívoros como zorros, coyotes y linces y los reptiles grandes como serpientes y cocodrilos" (`|MakeArray` "Continuar" :!type "Text")))
                  (switch `/Game/Blueprints/Enum_DialogueState` _state_4
                    (:`NewEnumerator0`
                      (bind _state_5 (`self.AddDialogue` "Letrero" "Se busca garantizar que los conejos estén en condiciones óptimas de salud y bienestar. De esta manera, se asegura que proporcionen la mejor nutrición posible a los depredadores que dependen de ellos para su recuperación y supervivencia" (`|MakeArray` "Continuar" :!type "Text")))
                      (switch `/Game/Blueprints/Enum_DialogueState` _state_5
                        (:`NewEnumerator0`
                          (bind _state_6 (`self.AddDialogue` "Letrero" "Gracias por tu interés y por apoyar la conservación de la vida silvestre" (`|MakeArray` "Continuar" :!type "Text")))
                          (switch `/Game/Blueprints/Enum_DialogueState` _state_6
                            (:`NewEnumerator0`
                              (`self.SetDialogueBranch` "Bunny")
                              (`self.CloseConversation`))))))))))))))
    (:`Bunny`
      (bind _state_7 (`self.AddDialogue` "Letrero" "Aquí y mas adelante se crían los conejos"))
      (switch `/Game/Blueprints/Enum_DialogueState` _state_7
        (:`NewEnumerator0`
          (`self.ClearDialogueProgress`)
          (`self.CloseConversation`))))))