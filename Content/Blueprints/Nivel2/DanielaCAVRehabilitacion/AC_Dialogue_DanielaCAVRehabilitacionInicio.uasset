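; Dialogue component for Daniela, who introduces the wildlife center's rehabilitation zone in Level 2 and assigns the animal-feeding task.
; The Dialogue override calls its parent, then switches on the active branch.
; The default branch chains Spanish lines on recovery times, aggression color codes and feeding parrots, hedgehogs and a snake, then switches to the Rehabilitacion branch.
; That branch repeats a reminder to fetch a bioterio mouse, clearing dialogue progress before closing.
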(fn `Dialogue`
  (`parent.Dialogue`)
  (switch `name` (`self.ActiveDialogueBranch`)
    (:`Default`
      (bind _state (`self.AddDialogue` "Daniela" "Bienvenido a la zona de rehabilitación del Centro de Atención y Valoración de Fauna Silvestre. Esta área es donde los animales se recuperan y se preparan para ser liberados de nuevo en su hábitat natural. Es un lugar crucial en nuestro proceso de rehabilitación y reintegración" (`|MakeArray` "Continuar" :!type "Text")))
      (switch `/Game/Blueprints/Enum_DialogueState` _state
        (:`NewEnumerator0`
          (bind _state_2 (`self.AddDialogue` "Daniela" "Aquí, cada especie tiene un tiempo específico de estadía que les permite recuperarse completamente antes de ser liberados: \nReptiles: 40 días \nMamíferos: 60 días \nPrimates: 90 días \nAves: 45 días \n" (`|MakeArray` "Continuar" :!type "Text")))
          (switch `/Game/Blueprints/Enum_DialogueState` _state_2
            (:`NewEnumerator0`
              (bind _state_3 (`self.AddDialogue` "Daniela" "Además, clasificamos a los animales según su nivel de agresividad para asegurar la seguridad tanto de los animales como del personal. Usamos un sistema de colores: \nVerde: Amigable \nAmarillo: Intermedio \nRojo: Peligroso \n" (`|MakeArray` "Continuar" :!type "Text")))
              (switch `/Game/Blueprints/Enum_DialogueState` _state_3
                (:`NewEnumerator0`
                  (bind _state_4 (`self.AddDialogue` "Daniela" "Es importante tener en cuenta que en esta área trabajamos con el objetivo de minimizar el contacto humano para que los animales puedan volver a su comportamiento natural y no dependan de nosotros cuando sean liberados" (`|MakeArray` "Continuar" :!type "Text")))
                  (switch `/Game/Blueprints/Enum_DialogueState` _state_4
                    (:`NewEnumerator0`
                      (bind _state_5 (`self.AddDialogue` "Daniela" "Un dato importante sobre la zona de rehabilitación es que mantenemos un monitoreo constante de cada animal. Esto nos permite ajustar sus dietas y cuidados según sus necesidades específicas, asegurando una recuperación completa y exitosa" (`|MakeArray` "Continuar" :!type "Text")))
                      (switch `/Game/Blueprints/Enum_DialogueState` _state_5
                        (:`NewEnumerator0`
                          (bind _state_6 (`self.AddDialogue` "Daniela" "Hoy necesitamos tu ayuda para alimentar a algunos de los animales en rehabilitación. En primer lugar, necesitamos alimentar a los loros. Estos coloridos pájaros son muy inteligentes y sociales, y requieren una dieta rica en frutas, semillas y vegetales frescos" (`|MakeArray` "Continuar" :!type "Text")))
                          (switch `/Game/Blueprints/Enum_DialogueState` _state_6
                            (:`NewEnumerator0`
                              (bind _state_7 (`self.AddDialogue` "Daniela" "Luego, tenemos que atender a nuestros erizos. A pesar de su apariencia espinosa, son animales fascinantes y requieren una dieta variada que incluya insectos, frutas y proteínas para mantenerse saludables" (`|MakeArray` "Continuar" :!type "Text")))
                              (switch `/Game/Blueprints/Enum_DialogueState` _state_7
                                (:`NewEnumerator0`
                                  (bind _state_8 (`self.AddDialogue` "Daniela" "Por último, necesitamos alimentar a una serpiente. Las serpientes son animales impresionantes y, en este caso, necesita una presa viva para su alimentación. Necesitarás ir a la zona de bioterio para buscar un ratón. Los ratones criados en el bioterio están en condiciones óptimas de salud y son una fuente de alimento adecuada para nuestros depredadores" (`|MakeArray` "Continuar" :!type "Text")))
                                  (switch `/Game/Blueprints/Enum_DialogueState` _state_8
                                    (:`NewEnumerator0`
                                      (`self.SetDialogueBranch` "Rehabilitacion")
                                      (`self.CloseConversation`))))))))))))))))))
    (:`Rehabilitacion`
      (bind _state_9 (`self.AddDialogue` "Daniela" "Alimenta a los animales, recuerda que debes ir por un ratón al bioterio"))
      (switch `/Game/Blueprints/Enum_DialogueState` _state_9
        (:`NewEnumerator0`
          (`self.ClearDialogueProgress`)
          (`self.CloseConversation`))))))