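; Dialogue component for Daniela's farewell at the end of the wildlife rescue and rehabilitation center (CAV) level, thanking the player in Spanish.
; It overrides Dialogue and switches on the active branch, with the default branch chaining single-option lines that advance on Pass Through.
; The last line switches the branch to FIN and closes the conversation.
; FIN repeats a reminder to head to the bus, then clears dialogue progress and closes.
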(fn `Dialogue`
  (`parent.Dialogue`)
  (switch `name` (`self.ActiveDialogueBranch`)
    (:`Default`
      (bind _state (`self.AddDialogue` "Daniela" "¡Hola de nuevo, rescatista! ¡Qué impresionante ha sido verte en acción hoy! Has demostrado un compromiso y una dedicación excepcionales hacia la fauna silvestre que cuidamos en nuestro centro" (`|MakeArray` "Continuar" :!type "Text")))
      (switch `/Game/Blueprints/Enum_DialogueState` _state
        (:`NewEnumerator0`
          (bind _state_2 (`self.AddDialogue` "Daniela" "Desde la evaluación inicial de los animales en el consultorio, pasando por el cuidado intensivo en el hospital, hasta la alimentación y el manejo en la zona de cuarentena y rehabilitación, tu trabajo ha sido esencial para el bienestar y la recuperación de estas criaturas vulnerables" (`|MakeArray` "Continuar" :!type "Text")))
          (switch `/Game/Blueprints/Enum_DialogueState` _state_2
            (:`NewEnumerator0`
              (bind _state_3 (`self.AddDialogue` "Daniela" "Cada tarea que has realizado, desde alimentar a los loros y erizos, hasta buscar alimento para nuestras serpientes en el bioterio, ha contribuido de manera significativa a nuestra misión de rescatar, rehabilitar y devolver a la vida silvestre a su estado natural" (`|MakeArray` "Continuar" :!type "Text")))
              (switch `/Game/Blueprints/Enum_DialogueState` _state_3
                (:`NewEnumerator0`
                  (bind _state_4 (`self.AddDialogue` "Daniela" "Es increíble ver cómo tu esfuerzo y dedicación impactan directamente en la vida de estos animales. Has sido una parte crucial de nuestro equipo, y tu compromiso con la conservación de la vida silvestre es verdaderamente inspirador" (`|MakeArray` "Continuar" :!type "Text")))
                  (switch `/Game/Blueprints/Enum_DialogueState` _state_4
                    (:`NewEnumerator0`
                      (bind _state_5 (`self.AddDialogue` "Daniela" "Ahora, es momento de despedirnos por hoy. Pero no te preocupes, tu aventura en pro de la fauna silvestre no termina aquí. Afuera, hay un autobús esperando para llevarte a tu próxima misión. Estamos seguros de que seguirás haciendo un trabajo increíble y ayudando a muchos más animales en tu camino" (`|MakeArray` "Continuar" :!type "Text")))
                      (switch `/Game/Blueprints/Enum_DialogueState` _state_5
                        (:`NewEnumerator0`
                          (bind _state_6 (`self.AddDialogue` "Daniela" "Gracias por todo tu esfuerzo y por ser parte de nuestra familia en el Centro de Atención y Valoración de Fauna Silvestre. ¡Sigue adelante con la misma pasión y compromiso, rescatista! " (`|MakeArray` "Continuar" :!type "Text")))
                          (switch `/Game/Blueprints/Enum_DialogueState` _state_6
                            (:`NewEnumerator0`
                              (bind _state_7 (`self.AddDialogue` "Daniela" "¡Nos vemos pronto y buena suerte en tu próxima aventura!" (`|MakeArray` "Continuar" :!type "Text")))
                              (switch `/Game/Blueprints/Enum_DialogueState` _state_7
                                (:`NewEnumerator0`
                                  (`self.SetDialogueBranch` "FIN")
                                  (`self.CloseConversation`))))))))))))))))
    (:`FIN`
      (bind _state_8 (`self.AddDialogue` "Daniela" "Dirígete al autobús para ir a tu próxima aventura "))
      (switch `/Game/Blueprints/Enum_DialogueState` _state_8
        (:`NewEnumerator0`
          (`self.ClearDialogueProgress`)
          (`self.CloseConversation`))))))