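; Dialogue component for the final bus interaction in Nivel2, asking the player in Spanish whether to end the adventure.
; Its Dialogue function calls the parent, then presents a two-option prompt through AddDialogue, branching on the returned state and chosen option.
; Confirming clears progress, closes the conversation and opens the Creditos level, while declining shows a short "another time" line before clearing and closing.
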(fn `Dialogue`
  (`parent.Dialogue`)
  (switch `name` (`self.ActiveDialogueBranch`)
    (:`Default`
      (bind (_state _optionindex) (`self.AddDialogue` "Tu" "Si uso el autobús ya no abra vuelta atrás. ¿Deseo terminar con la aventura?" (`|MakeArray` "Estoy listo" "Aún no me quiero ir" :!type "Text")))
      (switch `/Game/Blueprints/Enum_DialogueState` _state
        (:`NewEnumerator0`
          (switch `int` _optionindex
            (:`0`
              (`self.ClearDialogueProgress`)
              (`self.CloseConversation`)
              (`GameplayStatics.OpenLevel` "Creditos"))
            (:`1`
              (bind _state_2 (`self.AddDialogue` "Tu" "Será en otro momento"))
              (switch `/Game/Blueprints/Enum_DialogueState` _state_2
                (:`NewEnumerator0`
                  (`self.ClearDialogueProgress`)
                  (`self.CloseConversation`))))))))))