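; Dialogue component for María, who welcomes the player as a rescuer to the CAV wildlife care and assessment center in level 2.
; It overrides the Dialogue graph, switching on the active branch and chaining Spanish lines through their pass-through states.
; The default branch plays the introduction and directions to the clinic, then switches to the Consultorio branch.
; That branch repeats a short reminder to visit the clinic, clearing progress before closing the conversation.
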(fn `Dialogue`
  (`parent.Dialogue`)
  (switch `name` (`self.ActiveDialogueBranch`)
    (:`Default`
      (bind _state (`self.AddDialogue` "Maria" "¡Bienvenido al Centro de Atención y Valoración de Fauna Silvestre, rescatista! Qué alegría verte aquí y compartir esta experiencia contigo" (`|MakeArray` "Continuar" :!type "Text")))
      (switch `/Game/Blueprints/Enum_DialogueState` _state
        (:`NewEnumerator0`
          (bind _state_2 (`self.AddDialogue` "María" "En este lugar, nos dedicamos con pasión y compromiso al cuidado y rehabilitación de la vida silvestre. Es un honor contar con tu presencia, ya que tu labor como rescatista es fundamental para el bienestar de estas criaturas vulnerables" (`|MakeArray` "Continuar" :!type "Text")))
          (switch `/Game/Blueprints/Enum_DialogueState` _state_2
            (:`NewEnumerator0`
              (bind _state_3 (`self.AddDialogue` "María" "Debes dirigirte hacia el consultorio donde uno de nuestros expertos te explicará más detalladamente sobre el trabajo que realizamos aquí" (`|MakeArray` "Continuar" :!type "Text")))
              (switch `/Game/Blueprints/Enum_DialogueState` _state_3
                (:`NewEnumerator0`
                  (bind _state_4 (`self.AddDialogue` "María" "En el consultorio, podrás aprender sobre los procesos de evaluación médica, tratamiento y rehabilitación que llevamos a cabo para cada animal" (`|MakeArray` "Continuar" :!type "Text")))
                  (switch `/Game/Blueprints/Enum_DialogueState` _state_4
                    (:`NewEnumerator0`
                      (bind _state_5 (`self.AddDialogue` "María" "¡Adelante, te espera una nueva aventura en el mundo de la conservación de la vida silvestre!" (`|MakeArray` "Continuar" :!type "Text")))
                      (switch `/Game/Blueprints/Enum_DialogueState` _state_5
                        (:`NewEnumerator0`
                          (`self.SetDialogueBranch` "Consultorio")
                          (`self.CloseConversation`))))))))))))
    (:`Consultorio`
      (bind _state_6 (`self.AddDialogue` "María" "Ve al consultorio del CAV"))
      (switch `/Game/Blueprints/Enum_DialogueState` _state_6
        (:`NewEnumerator0`
          (`self.ClearDialogueProgress`)
          (`self.CloseConversation`))))))