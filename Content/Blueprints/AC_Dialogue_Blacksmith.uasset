(fn `Dialogue`
  (`parent.Dialogue`)
  (switch `name` (`self.ActiveDialogueBranch`)
    (:`Morning`
      (bind _state (`self.AddDialogue` "BlackSmith" "Good Morning" (`|MakeArray`)))
      (switch `/Game/Blueprints/Enum_DialogueState` _state
        (:`NewEnumerator0`
          (`self.ClearDialogueProgress`)
          (`self.CloseConversation`))))
    (:`Afternoon`
      (if (`self.bHasGivenBread?`)
        (bind _state_2 (`self.AddDialogue` "BlackSmith" "Thank u for the bread" (`|MakeArray`)))
        (switch `/Game/Blueprints/Enum_DialogueState` _state_2
          (:`NewEnumerator0`
            (`self.ClearDialogueProgress`)
            (`self.CloseConversation`)))
        (else
          (bind (_state_3 _optionindex) (`self.AddDialogue` "BlackSmith" "I would love a piece of bread, havent eaten the whole day, could you get me one?" (`|MakeArray` "Sure" "No dude, WTF" :!type "Text")))
          (switch `/Game/Blueprints/Enum_DialogueState` _state_3
            (:`NewEnumerator0`
              (switch `int` _optionindex
                (:`0`
                  (bind _state_4 (`self.AddDialogue` "BlackSmith" "Great, come speak to me when you have the bread" (`|MakeArray`)))
                  (switch `/Game/Blueprints/Enum_DialogueState` _state_4
                    (:`NewEnumerator0`
                      (if true
                        (bind (_state_5 _optionindex_2) (`self.AddDialogue` "BlackSmith" "Ahh, i see you have bread, give it to me quickly" (`|MakeArray` "Sure" "No" :!type "Text")))
                        (switch `/Game/Blueprints/Enum_DialogueState` _state_5
                          (:`NewEnumerator0`
                            (switch `int` _optionindex_2
                              (:`0`
                                (bind _state_6 (`self.AddDialogue` "BlackSmith" "You are so kind dude" (`|MakeArray`)))
                                (switch `/Game/Blueprints/Enum_DialogueState` _state_6
                                  (:`NewEnumerator0`
                                    (`self.ClearDialogueProgress`)
                                    (`self.CloseConversation`))
                                  (:`NewEnumerator1`
                                    (set `self.bHasGivenBread?` true))))
                              (:`1`
                                (bind _state_7 (`self.AddDialogue` "BlackSmith" "Oh okay, speak to me if you change your mind" (`|MakeArray`)))
                                (switch `/Game/Blueprints/Enum_DialogueState` _state_7
                                  (:`NewEnumerator0`
                                    (`self.RemoveDialogueProgress` 2)
                                    (`self.CloseConversation`)))))))
                        (else
                          (bind _state_8 (`self.AddDialogue` "BlackSmith" "come speak to me when you have the bread" (`|MakeArray`)))
                          (switch `/Game/Blueprints/Enum_DialogueState` _state_8
                            (:`NewEnumerator0`
                              (`self.RemoveDialogueProgress` 1)
                              (`self.CloseConversation`))))))))
                (:`1`
                  (bind _state_9 (`self.AddDialogue` "BlackSmith" "FUCKING IDIOT, btw speak to me again if  you change your mind jeje" (`|MakeArray`)))
                  (switch `/Game/Blueprints/Enum_DialogueState` _state_9
                    (:`NewEnumerator0`
                      (`self.ClearDialogueProgress`)
                      (`self.CloseConversation`))))))))))
    (:`Night`
      (bind _state_10 (`self.AddDialogue` "BlackSmith" "AAAAAH, I'm trying to sleep, leave me alone asshole" (`|MakeArray`)))
      (switch `/Game/Blueprints/Enum_DialogueState` _state_10
        (:`NewEnumerator0`
          (`self.ClearDialogueProgress`)
          (`self.CloseConversation`))))))

(fn `OpenConversation`
  (bind _interactioninstigator (message `/Game/Blueprints/BPI_Interactable.GetInteractionInstigator` (`self.GetOwner`)))
  (bind _asbp_player (cast `/Game/Blueprints/BP_Player` _interactioninstigator))
  (bind (_timeofday_days _timeofday_hours) (`KismetMathLibrary.BreakTimespan` (`/Game/Blueprints/BP_Player.TimeOfDay` _asbp_player)))
  (`self.SetDialogueBranch` (select `int` (+ (`KismetMathLibrary.Conv_BoolToInt` (and (>= _timeofday_hours 5) (< _timeofday_hours 15))) (* (`KismetMathLibrary.Conv_BoolToInt` (and (>= _timeofday_hours 15) (< _timeofday_hours 22))) 2)) :`0` "Night" :`1` "Morning" :`2` "Afternoon" :`3` "Default" :!type "Name"))
  (`parent.OpenConversation`))